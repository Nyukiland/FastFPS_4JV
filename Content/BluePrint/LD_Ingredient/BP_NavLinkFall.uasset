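; BP_NavLinkFall is a smart nav link that launches AI characters to the link's destination, judging by its name for drops between levels.
; On reach, CalculateVelo solves a ballistic velocity from JumpDuration and hardcoded gravity, which LaunchCharacter applies as a full override.
; During the jump, it disables the link and sets its NavModifier to a null area, restoring both after the delay.
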(event `self.ReceiveSmartLinkReached`
  (params (Agent :type "Actor Object Reference") (Destination :type "Vector Structure (by ref)"))
  (bind _jumpduration (`self.JumpDuration`))
  (bind _ascharacter (cast `Character` Agent))
  (`self.SetSmartLinkEnabled` false)
  (`NavModifierComponent.SetAreaClass` (`self.NavModifier`) "/Script/NavigationSystem.NavArea_Null")
  (bind _velocity (`self.CalculateVelo` Destination (`self.K2_GetActorLocation` Agent) _jumpduration))
  (`Character.LaunchCharacter` _ascharacter _velocity true true)
  (`KismetSystemLibrary.Delay` _jumpduration)
  (`self.SetSmartLinkEnabled` true)
  (`NavModifierComponent.SetAreaClass` (`self.NavModifier`) "/Script/NavigationSystem.NavArea_Default"))

(fn `CalculateVelo`
  (params (`Destination Location` :type "Vector Structure") (StartingLocation :type "Vector Structure") (Duration :type "Float (double-precision)"))
  (returns (Velocity :type "Vector Structure"))
  (locals (InDuration :type "Float (double-precision)"))
  (bind _induration (`local.InDuration`))
  (set `local.InDuration` Duration)
  (return (`KismetMathLibrary.MakeVector` (/ (- (.x `Destination Location`) (.x StartingLocation)) _induration) (/ (- (.y `Destination Location`) (.y StartingLocation)) _induration) (/ (- (.z `Destination Location`) (+ (.z StartingLocation) (* (`KismetMathLibrary.Square` (`local.InDuration`)) -0.5 982.0))) _induration))))

(fn `UserConstructionScript`)
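; BP_CheatControl is a possessable cheat controller that turns held-key chords into cheats and an easter egg.
; Key events mirror held letters and modifiers into booleans, which Tick checks while Right Shift is held.
; With Left Alt, holding the letters of YOGURT shows a widget until Tick sees the chord broken.
; Otherwise C+O+N kills all enemies through the enemy manager, and L repossesses BP_Player and destroys this actor.
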(event `self.ReceiveTick`
  (params (DeltaSeconds :type "Float (single-precision)"))
  (if (`self.Shift`)
    (if (`self.Alt`)
      (`self.EasterEgg`)
      (else
        (`self.Cheat`)
        (if (`self.L`)
          (bind _returnvalue (`GameplayStatics.GetActorOfClass` "/Game/BluePrint/Entity/BP_Player.BP_Player_C"))
          (`Controller.Possess` (`self.GetController`) _returnvalue)
          (`self.K2_DestroyActor` self))))))

(event `Key|A`
  (params (Key :type "Key Structure"))
  (:`Pressed`
    (set `self.A` true))
  (:`Released`
    (set `self.A` false)))

(event `Key|F`
  (params (Key :type "Key Structure"))
  (:`Pressed`
    (set `self.F` true))
  (:`Released`
    (set `self.F` false)))

(event `Key|K`
  (params (Key :type "Key Structure"))
  (:`Pressed`
    (set `self.K` true))
  (:`Released`
    (set `self.K` false)))

(event `Key|P`
  (params (Key :type "Key Structure"))
  (:`Pressed`
    (set `self.P` true))
  (:`Released`
    (set `self.P` false)))

(event `Key|U`
  (params (Key :type "Key Structure"))
  (:`Pressed`
    (set `self.U` true))
  (:`Released`
    (set `self.U` false)))

(event `Key|Z`
  (params (Key :type "Key Structure"))
  (:`Pressed`
    (set `self.Z` true))
  (:`Released`
    (set `self.Z` false)))

(event `Key|B`
  (params (Key :type "Key Structure"))
  (:`Pressed`
    (set `self.B` true))
  (:`Released`
    (set `self.B` false)))

(event `Key|G`
  (params (Key :type "Key Structure"))
  (:`Pressed`
    (set `self.G` true))
  (:`Released`
    (set `self.G` false)))

(event `Key|L`
  (params (Key :type "Key Structure"))
  (:`Pressed`
    (set `self.L` true))
  (:`Released`
    (set `self.L` false)))

(event `Key|Q`
  (params (Key :type "Key Structure"))
  (:`Pressed`
    (set `self.Q` true))
  (:`Released`
    (set `self.Q` false)))

(event `Key|V`
  (params (Key :type "Key Structure"))
  (:`Pressed`
    (set `self.V` true))
  (:`Released`
    (set `self.V` false)))

(event `Key|RightShift`
  (params (Key :type "Key Structure"))
  (:`Pressed`
    (set `self.Shift` true)
    (`KismetSystemLibrary.PrintString` "Hello"))
  (:`Released`
    (set `self.Shift` false)))

(event `Key|LeftAlt`
  (params (Key :type "Key Structure"))
  (:`Pressed`
    (set `self.Alt` true))
  (:`Released`
    (set `self.Alt` false)))

(event `Key|C`
  (params (Key :type "Key Structure"))
  (:`Pressed`
    (set `self.C` true))
  (:`Released`
    (set `self.C` false)))

(event `Key|H`
  (params (Key :type "Key Structure"))
  (:`Pressed`
    (set `self.H` true))
  (:`Released`
    (set `self.H` false)))

(event `Key|M`
  (params (Key :type "Key Structure"))
  (:`Pressed`
    (set `self.M` true))
  (:`Released`
    (set `self.M` false)))

(event `Key|R`
  (params (Key :type "Key Structure"))
  (:`Pressed`
    (set `self.R` true))
  (:`Released`
    (set `self.R` false)))

(event `Key|W`
  (params (Key :type "Key Structure"))
  (:`Pressed`
    (set `self.W` true))
  (:`Released`
    (set `self.W` false)))

(event `Key|D`
  (params (Key :type "Key Structure"))
  (:`Pressed`
    (set `self.D` true))
  (:`Released`
    (set `self.D` false)))

(event `Key|I`
  (params (Key :type "Key Structure"))
  (:`Pressed`
    (set `self.I` true))
  (:`Released`
    (set `self.I` false)))

(event `Key|N`
  (params (Key :type "Key Structure"))
  (:`Pressed`
    (set `self.N` true))
  (:`Released`
    (set `self.N` false)))

(event `Key|S`
  (params (Key :type "Key Structure"))
  (:`Pressed`
    (set `self.S` true))
  (:`Released`
    (set `self.S` false)))

(event `Key|X`
  (params (Key :type "Key Structure"))
  (:`Pressed`
    (set `self.X` true))
  (:`Released`
    (set `self.X` false)))

(event `Key|E`
  (params (Key :type "Key Structure"))
  (:`Pressed`
    (set `self.E` true))
  (:`Released`
    (set `self.E` false)))

(event `Key|J`
  (params (Key :type "Key Structure"))
  (:`Pressed`
    (set `self.J` true))
  (:`Released`
    (set `self.J` false)))

(event `Key|O`
  (params (Key :type "Key Structure"))
  (:`Pressed`
    (set `self.O` true))
  (:`Released`
    (set `self.O` false)))

(event `Key|T`
  (params (Key :type "Key Structure"))
  (:`Pressed`
    (set `self.T` true))
  (:`Released`
    (set `self.T` false)))

(event `Key|Y`
  (params (Key :type "Key Structure"))
  (:`Pressed`
    (set `self.Y` true))
  (:`Released`
    (set `self.Y` false)))

(fn `Cheat`
  (`self.KillAllEnemies`))

(fn `EasterEgg`
  (`self.YogurtEasterEgg`))

(fn `KillAllEnemies`
  (if (and (`self.C`) (`self.O`) (`self.N`))
    (bind _returnvalue (`FFEnemyManager.GetEnemyManager` self))
    (`FFEnemyManager.KillAllEnemies` _returnvalue)))

(fn `UserConstructionScript`)

(fn `YogurtEasterEgg`
  (bind _yogurtui (`self.YogurtUI`))
  (if (and (`self.Y`) (`self.O`) (`self.G`) (`self.U`) (`self.R`) (`self.T`))
    (`/Engine/EditorBlueprintResources/StandardMacros.DoOnce` false :!label _label
      (:`Completed`
        (bind _returnvalue (`|CreateWidget` "/Game/Interface/AllGood/W_YogurtEasterEgg.W_YogurtEasterEgg_C"))
        (bind _output_get (set `self.YogurtUI` _returnvalue))
        (`UserWidget.AddToViewport` _output_get 0)))
    (else
      (`|ExecutionSequence`
        (:`then_0`
          (goto _label :!via `Reset`))
        (:`then_1`
          (`/Engine/EditorBlueprintResources/StandardMacros.IsValid` _yogurtui
            (:`Is Valid`
              (`Widget.RemoveFromParent` _yogurtui)
              (set `self.YogurtUI` null)
              (`KismetSystemLibrary.CollectGarbage`))))))))
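; Player movement component for BP_Player, handling running, curve-driven multi-jumps, gravity and energy-limited sliding.
; Each tick feeds input, PlayerStats and ground checks into FFMovementBehavior, which applies the velocity.
; Coyote time and a short jump/slide buffer soften input timing; sliding shrinks the capsule, lowers the camera and allows steering.
; It also drives camera tilt, weapon animation flags and Wwise audio, including speed-based wind and enemy-proximity footstep volume.
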(event `DelayBegin`
  (bind _player (`self.Player`))
  (`|ExecutionSequence`
    (:`then_0`
      (bind _returnvalue (`GameplayStatics.GetActorOfClass` "/Game/BluePrint/Entity/BP_Player.BP_Player_C"))
      (set `self.Player` _returnvalue)
      (set `self.FFMovement` (`/Game/BluePrint/Entity/BP_Player.FFMovementBehavior` _player))
      (set `self.PlayerCol` (`/Game/BluePrint/Entity/BP_Player.PlayerCol` _player))
      (set `self.JumpTimer` (`.Jumpduration_32_1C23DAEB4D6A84A1976EE7BD5E54E9C6` (break `/Game/BluePrint/Data/S_PlayerStats` (`/Game/BluePrint/Entity/BP_Player.PlayerStats` (`self.Player`)))))
      (set `self.CanJumpCD` true)
      (set `self.SlideEnergy` (`.SlideEnergyMax_71_91A8C88B4566644F39D2F0B1E627DB58` (break `/Game/BluePrint/Data/S_PlayerStats` (`/Game/BluePrint/Entity/BP_Player.PlayerStats` (`self.Player`)))))
      (`AkGameplayStatics.PostEvent` "/Game/WwiseAudio/Events/Default_Work_Unit/behaviour/Wind.Wind")
      (`AkGameplayStatics.SetRTPCValue` "/Game/WwiseAudio/Game_Parameters/Default_Work_Unit/Wind_volume.Wind_volume"))
    (:`then_1`
      (add `/Game/BluePrint/Entity/BP_Player.SlideEventStarted` (`self.Player`) (delegate `SlideStart`))
      (add `/Game/BluePrint/Entity/BP_Player.SlideEventCancel` (`self.Player`) (delegate `SlideEnd`))
      (add `/Game/BluePrint/Entity/BP_Player.JumpEventStarted` (`self.Player`) (delegate `JumpCalled`)))))

(event `SlideStart`
  (bind (_movementspeed _movementspeedacceleration _movementspeeddeceleration _camerarotationspeed _fallgravitycurve _maxgravity _gravityspeed _slidemultiply _slideorientation _slideclampspeed _slideduration _slideaccelerationcurve _cameraspeedcurve _slidedeceleration _slideenergymax _slidecost) (break `/Game/BluePrint/Data/S_PlayerStats` (`/Game/BluePrint/Entity/BP_Player.PlayerStats` (`self.Player`))))
  ;[1 1 1] slide
  (if (>= (`self.SlideEnergy`) _slidecost)
    (if (and (not (`self.Jumping`)) (`self.Grounded`))
      (`CapsuleComponent.SetCapsuleHalfHeight` (`self.PlayerCol`) 40.0 true)
      (set `self.CallSlide` true)
      (`FFMathBlueprintHelper.DecrementFloat` (`self.SlideEnergy`) _slidecost)
      (else
        (set `self.Buffer` 2)
        (`self.BufferReset`)))))

(event `self.ReceiveEndPlay`
  (params (EndPlayReason :type "EEndPlayReason Enum" :default "Destroyed"))
  (clear `/Game/BluePrint/Entity/BP_Player.SlideEventCancel` (`self.Player`))
  (clear `/Game/BluePrint/Entity/BP_Player.SlideEventStarted` (`self.Player`))
  (clear `/Game/BluePrint/Entity/BP_Player.JumpEventStarted` (`self.Player`)))

(event `SlideEnd`
  ;[1 1 1] slide
  (if (`self.CallSlide`)
    (set `self.CallSlide` false)))

(event `JumpCalled`
  ;[1 1 1] Jump Call
  (if (`self.CanJumpCD`)
    (bind _jumpsuccess (`self.Call Jump`))
    (if (not _jumpsuccess)
      (set `self.Buffer` 1)
      (`self.BufferReset`))))

(event `JumpCD`
  ;[1 1 1] Jump Call
  (`KismetSystemLibrary.Delay` 0.1)
  (set `self.CanJumpCD` true))

(event `self.ReceiveTick`
  (params (DeltaSeconds :type "Float (single-precision)"))
  (`self.Movement`)
  (`self.MovementSound`)
  (`self.TiltCamera`)
  (`self.UpdateAnimator`))

(event `BufferReset`
  ;[1 1 1] Ugly buffer but will work (0 = nothing, 1 = jump, 2 = slide)
  (`KismetSystemLibrary.Delay` 0.3)
  (set `self.Buffer` 0))

(event `BufferCall`
  ;[1 1 1] Ugly buffer but will work (0 = nothing, 1 = jump, 2 = slide)
  (`KismetSystemLibrary.DelayUntilNextTick`)
  (if (!= (`self.Buffer`) 0)
    (switch `int` (`self.Buffer`)
      (:`1`
        ;;[1 1 1] event
        (`self.JumpCalled`))
      (:`2`
        (`self.SlideStart`)))
    (set `self.Buffer` 0)))

(fn `Call Jump`
  (returns (JumpSuccess :type Boolean))
  (locals (SlideJumpForce :type "Float (double-precision)" :default 10000.0))
  (bind (_movementspeed _movementspeedacceleration _movementspeeddeceleration _camerarotationspeed _fallgravitycurve _maxgravity _gravityspeed _slidemultiply _slideorientation _slideclampspeed _slideduration _slideaccelerationcurve _cameraspeedcurve _slidedeceleration _slideenergymax _slidecost _slideenergygainedperseconds _jumpaccelerationcurve _jumpduration _jumpvelo _jumpdurationslide _jumpveloslide _jumpcurveslide) (break `/Game/BluePrint/Data/S_PlayerStats` (`/Game/BluePrint/Entity/BP_Player.PlayerStats` (`self.Player`))))
  (bind (_movementspeed_2 _movementspeedacceleration_2 _movementspeeddeceleration_2 _camerarotationspeed_2 _fallgravitycurve_2 _maxgravity_2 _gravityspeed_2 _slidemultiply_2 _slideorientation_2 _slideclampspeed_2 _slideduration_2 _slideaccelerationcurve_2 _cameraspeedcurve_2 _slidedeceleration_2 _slideenergymax_2 _slidecost_2 _slideenergygainedperseconds_2 _jumpaccelerationcurve_2 _jumpduration_2 _jumpvelo_2 _jumpdurationslide_2 _jumpveloslide_2 _jumpcurveslide_2 _jumpsuccessives) (break `/Game/BluePrint/Data/S_PlayerStats` (`/Game/BluePrint/Entity/BP_Player.PlayerStats` (`self.Player`))))
  ;[1 1 1] Check if can Jump
  (if (and (`self.Grounded`) (not (`self.Jumping`)))
    (set `self.JumpCount` _jumpsuccessives)
    (elif (== _jumpsuccessives (`self.JumpCount`))
      (`/Engine/EditorBlueprintResources/StandardMacros.DecrementInt` (`self.JumpCount`)
        (:`  `
          _))))
  (if (> (`self.JumpCount`) 0)
    ;[1 1 1] Call Jump
    (`FFMathBlueprintHelper.DecrementInt` (`self.JumpCount`) 1)
    (set `self.JumpTimer` 0.0)
    (if (`self.IsSliding`)
      (set `self.JumpForce` _jumpveloslide)
      (set `self.JumpMaxTime` _jumpdurationslide)
      (set `self.JumpCurve` _jumpcurveslide)
      (else
        (set `self.JumpForce` _jumpvelo)
        (set `self.JumpMaxTime` _jumpduration)
        (set `self.JumpCurve` _jumpaccelerationcurve)))
    ;[1 1 1] CoolDown
    (set `self.CanJumpCD` false)
    (`self.JumpCD`)
    ;[1 1 1] Sound
    (`AkGameplayStatics.PostEvent` "/Game/WwiseAudio/Events/Default_Work_Unit/behaviour/JUMP.JUMP")
    (return true)
    (else
      (return false))))

(fn `GetClosestEnemy`
  (returns (Dist :type "Float (double-precision)"))
  (locals (Distance :type "Float (double-precision)" :default 100000.0))
  (bind _returnvalue (`FFEnemyControl.GetEnemyControl` self))
  (bind _returnvalue_2 (`FFEnemyControl.GetAllEnemies` _returnvalue))
  (for _array_element _returnvalue_2
    (bind _asbp_base_enemy (cast `/Game/BluePrint/Entity/Enemy/BP_BaseEnemy` _array_element))
    (bind _returnvalue_3 (`KismetMathLibrary.Vector_Distance` (`SceneComponent.K2_GetComponentLocation` (`Character.CapsuleComponent` _asbp_base_enemy)) (`SceneComponent.K2_GetComponentLocation` (`/Game/BluePrint/Entity/BP_Player.PlayerCol` (`self.Player`)))))
    (if (< _returnvalue_3 (`local.Distance`))
      (set `local.Distance` _returnvalue_3)))
  (return (`local.Distance`)))

(fn `GravityBehavior`
  (returns (GroundHit :type "HitResult Structure"))
  (locals (TraceSize :type "Float (double-precision)"))
  (bind (_movementspeed _movementspeedacceleration _movementspeeddeceleration _camerarotationspeed _fallgravitycurve _maxgravity _gravityspeed) (break `/Game/BluePrint/Data/S_PlayerStats` (`/Game/BluePrint/Entity/BP_Player.PlayerStats` (`self.Player`))))
  (if (`self.IsSliding`)
    (set `local.TraceSize` 65.0)
    (else
      (set `local.TraceSize` 85.0)))
  (bind _groundhit (`FFMovementBehavior.GroundCheckGravity` (`self.FFMovement`) _maxgravity _fallgravitycurve (`self.GravityTimer`) _gravityspeed (`local.TraceSize`))
    (:`Grounded`
      (if (not (`self.Grounded`))
        (`AkGameplayStatics.PostEvent` "/Game/WwiseAudio/Events/Default_Work_Unit/behaviour/land.land"))
      ;[1 1 1] Coyote Time
      (`self.BufferCall`)
      (set `self.CoyoteTimer` 0.0)
      (set `self.Grounded` true)
      ;[1 1 1] Gravity Timer
      (set `self.GravityTimer` 0.0)
      (return _groundhit))
    (:`NotGrounded`
      (bind _returnvalue (`FFMathBlueprintHelper.IncrementFloat` (`self.CoyoteTimer`) (`GameplayStatics.GetWorldDeltaSeconds`)))
      (if (> _returnvalue (`self.CoyoteTimeMax`))
        (set `self.Grounded` false))
      (if (not (`self.Jumping`))
        (`FFMathBlueprintHelper.IncrementFloat` (`self.GravityTimer`) (`GameplayStatics.GetWorldDeltaSeconds`))
        (`FFMathBlueprintHelper.ClampFloatByRef` (`self.GravityTimer`) 0.0 _gravityspeed)
        (return _groundhit)))))

(fn `Jump`
  (if (< (`self.JumpTimer`) (`self.JumpMaxTime`))
    (`FFMovementBehavior.JumpBehavior` (`self.FFMovement`) (`self.JumpForce`) (`self.JumpCurve`) (`self.JumpMaxTime`) (`self.JumpTimer`))
    (set `self.Jumping` true)
    (`FFMathBlueprintHelper.IncrementFloat` (`self.JumpTimer`) (`GameplayStatics.GetWorldDeltaSeconds`))
    (else
      (set `self.Jumping` false)))
  (return))

(fn `Movement`
  (locals (GroundHit :type "HitResult Structure"))
  (bind _ffmovement (`self.FFMovement`))
  (bind (_movementspeed _movementspeedacceleration _movementspeeddeceleration _camerarotationspeed _fallgravitycurve _maxgravity _gravityspeed _slidemultiply _slideorientation _slideclampspeed _slideduration _slideaccelerationcurve _cameraspeedcurve _slidedeceleration _slideenergymax _slidecost _slideenergygainedperseconds _jumpaccelerationcurve _jumpduration _jumpvelo _jumpdurationslide _jumpveloslide _jumpcurveslide _jumpsuccessives _jumpair_inertiadeceleration _jumpmaxinertia _jumpaircontrol) (break `/Game/BluePrint/Data/S_PlayerStats` (`/Game/BluePrint/Entity/BP_Player.PlayerStats` (`self.Player`))))
  (bind (_movementspeed_2 _movementspeedacceleration_2 _movementspeeddeceleration_2) (break `/Game/BluePrint/Data/S_PlayerStats` (`/Game/BluePrint/Entity/BP_Player.PlayerStats` (`self.Player`))))
  (`FFMovementBehavior.GetMovement` (`self.FFMovement`) (`self.PlayerCol`) (`/Game/BluePrint/Entity/BP_Player.Camera` (`self.Player`)))
  (bind _groundhit (`self.GravityBehavior`))
  (set `local.GroundHit` _groundhit)
  (if (and (`self.Grounded`) (not (`self.Jumping`)))
    ;[1 1 1] Move
    (if (not (`self.IsSliding`))
      (`FFMovementBehavior.MoveInDirection` _ffmovement (`/Game/BluePrint/Entity/BP_Player.InputMove` (`self.Player`)) _movementspeedacceleration_2 _movementspeeddeceleration_2 _movementspeed_2
        (:`NotInUse`
          _)
        (:`InUse`
          _))
      (else
        (`FFMovementBehavior.MoveInDirection` _ffmovement (`/Game/BluePrint/Entity/BP_Player.InputMove` (`self.Player`)) (`self.AccelerationCrouch`) (`.Slidedeceleration_25_DC16679F4230902AB682B4BADC875836` (break `/Game/BluePrint/Data/S_PlayerStats` (`/Game/BluePrint/Entity/BP_Player.PlayerStats` (`self.Player`)))) (`self.MaxSpeedCrouch`)
          (:`NotInUse`
            _)
          (:`InUse`
            _))))
    (else
      (`FFMovementBehavior.MoveInDirection` (`self.FFMovement`) (`/Game/BluePrint/Entity/BP_Player.InputMove` (`self.Player`)) _jumpaircontrol _jumpair_inertiadeceleration _jumpmaxinertia
        (:`NotInUse`
          _)
        (:`InUse`
          _))))
  (`self.Slide` (`local.GroundHit`))
  (`self.Jump`)
  (bind _hitroof (`FFMovementBehavior.GiveVelocity` (`self.FFMovement`) (`self.Grounded`) (`.ImpactNormal` (`GameplayStatics.BreakHitResult` (`local.GroundHit`))) (0.0 0.0 0.0) 100.0))
  (if _hitroof
    (set `self.JumpTimer` (`self.JumpMaxTime`)))
  (return))

(fn `MovementSound`
  (bind _returnvalue (- (`KismetMathLibrary.VSize` (`FFMovementBehavior.CurVelocity` (`/Game/BluePrint/Entity/BP_Player.FFMovementBehavior` (`self.Player`)))) 825.0))
  ;[1 1 1] Wind
  (if (< _returnvalue 0.0)
    (`AkGameplayStatics.SetRTPCValue` "/Game/WwiseAudio/Game_Parameters/Default_Work_Unit/Wind_volume.Wind_volume")
    (else
      (`AkGameplayStatics.SetRTPCValue` "/Game/WwiseAudio/Game_Parameters/Default_Work_Unit/Wind_volume.Wind_volume" (* (`KismetMathLibrary.FClamp` (/ _returnvalue (- 1350.0 825.0))) 100.0))))
  ;[1 1 1] footStep
  ;;[1 1 1] volume down when enemy close
  (bind _dist (`self.GetClosestEnemy`))
  (`AkGameplayStatics.SetRTPCValue` "/Game/WwiseAudio/Game_Parameters/Default_Work_Unit/Footsteps_Volume.Footsteps_Volume" (* (`KismetMathLibrary.FClamp` (/ _dist 750.0)) 100.0))
  (if (and (not (== (`/Game/BluePrint/Entity/BP_Player.InputMove` (`self.Player`)) (0.0 0.0))) (`self.Grounded`) (not (`/Game/BluePrint/Entity/BP_Player.InputSlide` (`self.Player`))))
    (bind _returnvalue_2 (`FFMathBlueprintHelper.IncrementFloat` (`self.MovementSoundTimer`) (`GameplayStatics.GetWorldDeltaSeconds`)))
    (if (> _returnvalue_2 0.4)
      (`AkGameplayStatics.PostEvent` "/Game/WwiseAudio/Events/Default_Work_Unit/behaviour/RUN.RUN")
      (set `self.MovementSoundTimer` 0.0))
    (else
      (set `self.MovementSoundTimer` 0.4))))

(fn `Slide`
  (params (Hit :type "HitResult Structure"))
  (locals (SlideHeightToGo :type "Float (double-precision)") (pivotPrevLocation :type "Vector Structure"))
  (bind _playercol (`self.PlayerCol`))
  (bind _ffmovement (`self.FFMovement`))
  (bind (_inputmove_x _inputmove_y) (`KismetMathLibrary.BreakVector2D` (`/Game/BluePrint/Entity/BP_Player.InputMove` (`self.Player`))))
  (bind _pivot (`/Game/BluePrint/Entity/BP_Player.Pivot` (`self.Player`)))
  (bind (_movementspeed _movementspeedacceleration _movementspeeddeceleration _camerarotationspeed _fallgravitycurve _maxgravity _gravityspeed _slidemultiply _slideorientation _slideclampspeed _slideduration _slideaccelerationcurve _cameraspeedcurve _slidedeceleration _slideenergymax _slidecost _slideenergygainedperseconds) (break `/Game/BluePrint/Data/S_PlayerStats` (`/Game/BluePrint/Entity/BP_Player.PlayerStats` (`self.Player`))))
  (bind (_relativelocation_x _relativelocation_y _relativelocation_z) (`KismetMathLibrary.BreakVector` (`SceneComponent.RelativeLocation` _pivot)))
  (if (`self.IsSliding`)
    ;[1 1 1] LerpCam
    (set `local.SlideHeightToGo` -300.0)
    (else
      (set `local.SlideHeightToGo` 200.0)))
  (`SceneComponent.K2_SetRelativeLocation` _pivot (`KismetMathLibrary.MakeVector` 0.0 0.0 (`KismetMathLibrary.FClamp` (+ _relativelocation_z (* (- (`local.SlideHeightToGo`) _relativelocation_z) (`GameplayStatics.GetWorldDeltaSeconds`) (`self.CamCrouchSpeed`))) -10.0 40.0)) false false)
  ;[1 1 1] Slide Energy
  (`FFMathBlueprintHelper.IncrementFloat` (`self.SlideEnergy`) (* _slideenergygainedperseconds (`GameplayStatics.GetWorldDeltaSeconds`)))
  (`FFMathBlueprintHelper.ClampFloatByRef` (`self.SlideEnergy`) 0.0 _slideenergymax)
  (`FFMovementBehavior.Slide` (`self.FFMovement`) (`self.CallSlide`) _slidemultiply _slideclampspeed _slideaccelerationcurve _slideduration (`.ImpactNormal` (`GameplayStatics.BreakHitResult` Hit))
    (:`NotInUse`
      ;[1 1 1] Slide Action
      (if (`self.IsSliding`)
        (if (`self.Grounded`)
          (set `self.IsSliding` false)
          (set `self.CallSlide` false)
          (`CapsuleComponent.SetCapsuleHalfHeight` _playercol 80.0 true)
          (set `local.pivotPrevLocation` (`SceneComponent.K2_GetComponentLocation` (`/Game/BluePrint/Entity/BP_Player.Pivot` (`self.Player`))))
          (`SceneComponent.K2_AddWorldOffset` _playercol (0.0 0.0 10.0) false false)
          (`SceneComponent.K2_SetWorldLocation` (`/Game/BluePrint/Entity/BP_Player.Pivot` (`self.Player`)) (`local.pivotPrevLocation`) false false)
          (set `self.StoredSlideDir` (0.0 0.0 0.0))
          (`AkGameplayStatics.SetState` "/Game/WwiseAudio/States/Default_Work_Unit/Slide_state/Slide_state-end.Slide_state-end")
          (`AkGameplayStatics.PostEvent` "/Game/WwiseAudio/Events/Default_Work_Unit/behaviour/Slide_End.Slide_End")
          (`AkGameplayStatics.SetRTPCValue` "/Game/WwiseAudio/Game_Parameters/Default_Work_Unit/Slide_Volume.Slide_Volume" 100.0)
          (else
            (if (== (`self.StoredSlideDir`) (0.0 0.0 0.0)) :!label _label
              (set `self.StoredSlideDir` (`FFMovementBehavior.SlideDir` (`self.FFMovement`))))
            (set `FFMovementBehavior.SlideDir` (+ (`self.StoredSlideDir`) (* _inputmove_y (* (`.SlideOrientation_91_19C45F7F48F2AC0C19359D97CFA71402` (break `/Game/BluePrint/Data/S_PlayerStats` (`/Game/BluePrint/Entity/BP_Player.PlayerStats` (`self.Player`)))) -1.0) (`KismetMathLibrary.Normal` (`KismetMathLibrary.Cross_VectorVector` (`KismetMathLibrary.Normal` (`FFMovementBehavior.SlideDir` (`self.FFMovement`))) (0.0 0.0 1.0))))) (`self.FFMovement`))
            (if (not (`self.IsSliding`))
              (`AkGameplayStatics.SetState` "/Game/WwiseAudio/States/Default_Work_Unit/Slide_state/Slide_state-loop.Slide_state-loop")
              (`AkGameplayStatics.PostEvent` "/Game/WwiseAudio/Events/Default_Work_Unit/behaviour/Slide_Loop.Slide_Loop"))
            (set `self.IsSliding` true)))
        (return)))
    (:`InUse`
      (if (`self.Grounded`)
        (`AkGameplayStatics.SetRTPCValue` "/Game/WwiseAudio/Game_Parameters/Default_Work_Unit/Slide_Volume.Slide_Volume" 100.0)
        (goto _label)
        (else
          (`AkGameplayStatics.SetRTPCValue` "/Game/WwiseAudio/Game_Parameters/Default_Work_Unit/Slide_Volume.Slide_Volume" 0.0 100)
          (`FFMovementBehavior.AddExternalForce` _ffmovement (* (`KismetMathLibrary.Normal` (`KismetMathLibrary.MakeVector` (.x (`FFMovementBehavior.CurVelocity` _ffmovement)) (.y (`FFMovementBehavior.CurVelocity` _ffmovement)))) (`.SlideJumpPropulsion_88_F7254D0A48B0A3AF52A4A1A084733736` (break `/Game/BluePrint/Data/S_PlayerStats` (`/Game/BluePrint/Entity/BP_Player.PlayerStats` (`self.Player`))))))
          (goto _label))))))

(fn `TiltCamera`
  (locals (MaxTilt :type "Float (double-precision)" :default 2.0))
  (bind _player (`self.Player`))
  (bind _maxtilt (`local.MaxTilt`))
  (bind _camera (`/Game/BluePrint/Entity/BP_Player.Camera` _player))
  (bind (_inputmove_x _inputmove_y) (`KismetMathLibrary.BreakVector2D` (`/Game/BluePrint/Entity/BP_Player.InputMove` _player)))
  (bind _relativerotation_roll (`KismetMathLibrary.BreakRotator` (`SceneComponent.RelativeRotation` _camera)))
  (`SceneComponent.K2_SetRelativeRotation` _camera (`KismetMathLibrary.MakeRotator` (/ (`KismetMathLibrary.Conv_IntToDouble` (`KismetMathLibrary.Round` (* (`KismetMathLibrary.FClamp` (+ _relativerotation_roll (* (- (* _inputmove_y (`local.MaxTilt`)) _relativerotation_roll) 0.3)) (* _maxtilt -1.0) _maxtilt) 10.0))) 10.0)) false false))

(fn `UpdateAnimator`
  (bind (_curvelocity_x _curvelocity_y) (`KismetMathLibrary.BreakVector` (`FFMovementBehavior.CurVelocity` (`self.FFMovement`))))
  (if (`|EnumInequality` (`/Game/BluePrint/Entity/BP_WeaponComponent.WeaponName` (`/Game/BluePrint/Entity/BP_Player.BP_WeaponComponent` (`self.Player`))) "NewEnumerator2")
    (bind _asfps_weapon_skeleton_anim_blueprint (cast `/Game/FBX/FPS_Weapon_Skeleton_AnimBlueprint` (`SkeletalMeshComponent.GetAnimInstance` (`/Game/BluePrint/Weapon/BP_WeaponBase.SkeletalMesh` (`/Game/BluePrint/Entity/BP_WeaponComponent.CurrentWeapon` (`/Game/BluePrint/Entity/BP_Player.BP_WeaponComponent` (`self.Player`)))))))
    (set `/Game/FBX/FPS_Weapon_Skeleton_AnimBlueprint.IsSliding` (`self.IsSliding`) _asfps_weapon_skeleton_anim_blueprint)
    (set `/Game/FBX/FPS_Weapon_Skeleton_AnimBlueprint.IsWalking` (not (<= (`KismetMathLibrary.VSize2D` (`KismetMathLibrary.MakeVector2D` _curvelocity_x _curvelocity_y)) 0.0)) _asfps_weapon_skeleton_anim_blueprint)))
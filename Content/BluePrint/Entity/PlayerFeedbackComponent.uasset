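; Player feedback component that adjusts the player camera's field of view according to movement speed to convey a sense of velocity.
; On BeginPlay it finds BP_Player and seeds the current FOV.
; Every tick it normalizes the movement behavior's velocity against a max speed, remaps it through an FOV curve into a clamped range, and smooths toward that target before applying it to the camera.
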(event `self.ReceiveBeginPlay`
  (bind _returnvalue (`GameplayStatics.GetActorOfClass` "/Game/BluePrint/Entity/BP_Player.BP_Player_C"))
  (set `self.Player` _returnvalue)
  (set `self.CurFOV` 90.0))

(event `self.ReceiveTick`
  (params (DeltaSeconds :type "Float (single-precision)"))
  (`self.SpeedFeedback`))

(fn `SpeedFeedback`
  (locals (LowerRange :type "Float (double-precision)" :default 90.0) (TopRange :type "Float (double-precision)" :default 130.0) (MinSpeed :type "Float (double-precision)") (MaxSpeed :type "Float (double-precision)" :default 2000.0))
  (bind _returnvalue (`FFBlueprintHelper.EvaluateCurve` "/Game/Curve/FC_FOVCurve.FC_FOVCurve" (`KismetMathLibrary.FClamp` (/ (`KismetMathLibrary.VSize` (`FFMovementBehavior.CurVelocity` (`/Game/BluePrint/Entity/BP_Player.FFMovementBehavior` (`self.Player`)))) (`local.MaxSpeed`)))))
  (bind _returnvalue_2 (`FFBlueprintHelper.SmoothValueByRef` (`self.CurFOV`) (`KismetMathLibrary.FClamp` (`KismetMathLibrary.Conv_IntToDouble` (`KismetMathLibrary.Round` (`KismetMathLibrary.Lerp` (`local.LowerRange`) (`local.TopRange`) _returnvalue))) (`local.LowerRange`) (`local.TopRange`)) 1.0 (`GameplayStatics.GetWorldDeltaSeconds`)))
  (`CameraComponent.SetFieldOfView` (`/Game/BluePrint/Entity/BP_Player.Camera` (`self.Player`)) _returnvalue_2))
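; BP_Player is the player character, spawning or finding the menu manager, registering with enemy control and routing input to movement and weapon components.
; Holding heal drains weapon combo on looping timers to gain a life, while damage triggers brief invincibility or death.
; Tick smooths look rotation, sums speed, shot, laser and heal FOV offsets, and sets Wwise music phases from nearby enemy count.
; Timelines, camera shakes and post-process parameters drive game feel.
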(event `self.ReceiveBeginPlay`
  ;[1 1 1] Add UI
  (bind _returnvalue (`GameplayStatics.GetActorOfClass` "/Game/BluePrint/Data/BP_MenuManager.BP_MenuManager_C"))
  (`/Engine/EditorBlueprintResources/StandardMacros.IsValid` _returnvalue
    (:`Is Valid`
      (set `self.MenuManager` _returnvalue)
      (`/Game/BluePrint/Data/BP_MenuManager.InitMenus` (`self.MenuManager`) self))
    (:`Is Not Valid`
      (bind _returnvalue_2 (`|SpawnActorFromClass` "/Game/BluePrint/Data/BP_MenuManager.BP_MenuManager_C" (`KismetMathLibrary.MakeTransform` (0.0 0.0 0.0)) "Undefined" "MultiplyWithRoot" null null))
      (set `self.MenuManager` _returnvalue_2)
      (`/Game/BluePrint/Data/BP_MenuManager.InitMenus` (`self.MenuManager`) self)
      (set `/Game/BluePrint/Entity/BP_WeaponComponent.Crosshair` (`/Game/BluePrint/Data/BP_MenuManager.Crosshair` (`self.MenuManager`)) (`self.BP_WeaponComponent`))))
  (`/Game/BluePrint/Entity/BP_WeaponComponent.InitWeapons` (`self.BP_WeaponComponent`))
  (if (`self.LaunchMenu`)
    (`/Game/BluePrint/Data/BP_MenuManager.StopGame` (`self.MenuManager`))
    (`/Game/BluePrint/Data/BP_MenuManager.ShowMenus` (`self.MenuManager`))
    (else
      (`/Game/BluePrint/Data/BP_MenuManager.StartGame` (`self.MenuManager`))))
  (bind _output_get (set `self.CurrentFOV` 95.0))
  (`CameraComponent.SetFieldOfView` (`self.Camera`) _output_get)
  (set `self.CamPos` (`SceneComponent.RelativeLocation` (`self.Camera`)))
  (set `self.BasePostPro` (`CameraComponent.PostProcessSettings` (`self.Camera`)))
  (set `self.CurrentCamRot` (`.CameraRotationspeed_50_6B0B5B424D2351040BA9DCBDB3C2FCEF` (break `/Game/BluePrint/Data/S_PlayerStats` (`self.PlayerStats`))))
  (bind _returnvalue_3 (`FFEnemyControl.GetEnemyControl` self))
  (bind _output_get_2 (set `self.EnemyControl` _returnvalue_3))
  (`FFEnemyControl.RegisterPlayer` _output_get_2 self)
  (`AkGameplayStatics.SetState` "/Game/WwiseAudio/States/Default_Work_Unit/Music/Music-Phase_1.Music-Phase_1")
  (`AkGameplayStatics.PostEvent` "/Game/WwiseAudio/Events/Default_Work_Unit/Music.Music")
  (set `self.StartPos` (`SceneComponent.K2_GetComponentLocation` (`self.PlayerCol`))))

(event `self.ReceiveTick`
  (params (DeltaSeconds :type "Float (single-precision)"))
  (bind (_returnvalue_x _returnvalue_y) (`KismetMathLibrary.BreakVector2D` (`|GetInputActionValue`)))
  (bind (_clampy_x _clampy_y) (`KismetMathLibrary.BreakVector` (`self.ClampY`)))
  (bind _output_get (set `self.CurrentGoTOCamRot` (* (`.CameraRotationspeed_50_6B0B5B424D2351040BA9DCBDB3C2FCEF` (break `/Game/BluePrint/Data/S_PlayerStats` (`self.PlayerStats`))) (`/Game/BluePrint/Entity/BP_WeaponComponent.RotationFactor` (`self.BP_WeaponComponent`)))))
  (bind _returnvalue (`FFBlueprintHelper.SmoothValueByRef` (`self.CurrentCamRot`) _output_get (`.SmoothRotation_54_4EE18B7540BB2C93A8775DA2EC4AED7C` (break `/Game/BluePrint/Data/S_Weapon` (`/Game/BluePrint/Weapon/BP_WeaponBase.WeaponData` (`/Game/BluePrint/Entity/BP_WeaponComponent.CurrentWeapon` (`self.BP_WeaponComponent`))))) DeltaSeconds))
  (`FFShootRelatedBehavior.LookAround` (`self.FFShootRelatedBehavior`) (`self.Pivot`) (`self.PivotY`) _returnvalue (`KismetMathLibrary.MakeVector` _returnvalue_y _returnvalue_x) _clampy_x _clampy_y)
  (set `self.InputMove` (`|GetInputActionValue`))
  (set `self.InputSlide` (`|GetInputActionValue`))
  (bind _fov (`self.Speed Feed Back`))
  (`CameraComponent.SetFieldOfView` (`self.Camera`) (+ (+ (+ _fov (`self.ShootFOV`)) (`self.ShootFOVNiveau`)) (`self.HealFOV`)))
  (`self.Music`))

(event `EnhancedInput|/Game/Input/IA_Jump`
  (params (ActionValue :type Boolean) (ElapsedSeconds :type "Float (double-precision)") (TriggeredSeconds :type "Float (double-precision)") (InputAction :type "InputAction Object Reference" :default "/Game/Input/IA_Jump.IA_Jump"))
  (:`Started`
    (if (not (`self.UsingLifeGain`))
      (`self.JumpEventStarted`))))

(event `EnhancedInput|/Game/Input/IA_Shoot2`
  (params (ActionValue :type Boolean) (ElapsedSeconds :type "Float (double-precision)") (TriggeredSeconds :type "Float (double-precision)") (InputAction :type "InputAction Object Reference" :default "/Game/Input/IA_Shoot2.IA_Shoot2"))
  ;[1 1 1] Weapons
  (:`Triggered`
    (if (not (`self.UsingLifeGain`))
      (`/Game/BluePrint/Entity/BP_WeaponComponent.SetLaserEndPoint` (`self.BP_WeaponComponent`))))
  (:`Started`
    (if (not (`self.UsingLifeGain`))
      (set `/Game/BluePrint/Entity/BP_WeaponComponent.IsHolding` true (`self.BP_WeaponComponent`))
      (`/Game/BluePrint/Entity/BP_WeaponComponent.Change To` (`self.BP_WeaponComponent`) "NewEnumerator1")))
  (:`Completed`
    (if (not (`self.UsingLifeGain`))
      (set `/Game/BluePrint/Entity/BP_WeaponComponent.IsHolding` false (`self.BP_WeaponComponent`))
      (`/Game/BluePrint/Entity/BP_WeaponComponent.Change To` (`self.BP_WeaponComponent`) "NewEnumerator0"))))

(event `EnhancedInput|/Game/Input/IA_ChangeWeapon`
  (params (ActionValue :type "Float (double-precision)") (ElapsedSeconds :type "Float (double-precision)") (TriggeredSeconds :type "Float (double-precision)") (InputAction :type "InputAction Object Reference" :default "/Game/Input/IA_ChangeWeapon.IA_ChangeWeapon"))
  ;[1 1 1] Weapons
)

(event `EnhancedInput|/Game/Input/IA_GainLife`
  (params (ActionValue :type Boolean) (ElapsedSeconds :type "Float (double-precision)") (TriggeredSeconds :type "Float (double-precision)") (InputAction :type "InputAction Object Reference" :default "/Game/Input/IA_GainLife.IA_GainLife"))
  ;[1 1 1] Weapons
  (:`Started`
    (`self.StartLifeGain`))
  (:`Completed`
    (`self.StopLifeGain`)))

(event `EnhancedInput|/Game/Input/IA_Slide`
  (params (ActionValue :type Boolean) (ElapsedSeconds :type "Float (double-precision)") (TriggeredSeconds :type "Float (double-precision)") (InputAction :type "InputAction Object Reference" :default "/Game/Input/IA_Slide.IA_Slide"))
  (:`Started`
    (if (not (`self.UsingLifeGain`))
      (`self.SlideEventStarted`)))
  (:`Canceled`
    (if (not (`self.UsingLifeGain`)) :!label _label
      (`self.SlideEventCancel`)))
  (:`Completed`
    (goto _label)))

(event `EnhancedInput|/Game/Input/IA_Shoot1`
  (params (ActionValue :type Boolean) (ElapsedSeconds :type "Float (double-precision)") (TriggeredSeconds :type "Float (double-precision)") (InputAction :type "InputAction Object Reference" :default "/Game/Input/IA_Shoot1.IA_Shoot1"))
  ;[1 1 1] Weapons
  (:`Triggered`
    (if (not (`self.UsingLifeGain`))
      (`/Game/BluePrint/Entity/BP_WeaponComponent.Shoot 1` (`self.BP_WeaponComponent`)))))

(event `EnhancedInput|/Game/Input/IA_Reload`
  (params (ActionValue :type Boolean) (ElapsedSeconds :type "Float (double-precision)") (TriggeredSeconds :type "Float (double-precision)") (InputAction :type "InputAction Object Reference" :default "/Game/Input/IA_Reload.IA_Reload"))
  ;[1 1 1] Weapons
  (:`Started`
    (if (not (`self.UsingLifeGain`))
      (`/Game/BluePrint/Entity/BP_WeaponComponent.Reload` (`self.BP_WeaponComponent`)))))

(event `StartLifeGain`
  (bind _currentcombopercentage (`/Game/BluePrint/Entity/BP_WeaponComponent.CurrentComboPercentage` (`self.BP_WeaponComponent`)))
  ;[1 0.4603 0.9097] Heal
  (if (and (>= _currentcombopercentage 33.0) (`/Game/BluePrint/Entity/BP_MovementComponenet.Grounded` (`self.BP_MovementComponent`)) (not (`/Game/BluePrint/Entity/BP_WeaponComponent.IsLaserOn` (`self.BP_WeaponComponent`))) (< (`self.PlayerLife`) (`self.PlayerMaxLife`)))
    (set `self.StartHealPercentage` _currentcombopercentage)
    (set `self.UsingLifeGain` true)
    (`/Game/Interface/W_Crosshair.ToggleHealFeedback` (`/Game/BluePrint/Data/BP_MenuManager.Crosshair` (`self.MenuManager`)) true)
    (`self.HealStart`)
    (bind _returnvalue (`KismetSystemLibrary.K2_SetTimerDelegate` (delegate `GainLife`) (`.TimerHeal_94_DB4581B743209148858C4FA1143E08CB` (break `/Game/BluePrint/Data/S_PlayerStats` (`self.PlayerStats`)))))
    (bind _returnvalue_2 (`KismetSystemLibrary.K2_SetTimerDelegate` (delegate `DecreaseComboValue`) 0.1 true))))

(event `StopLifeGain`
  ;[1 0.4603 0.9097] Heal
  (`self.HealCancel`)
  (`self.ClearHealBind`)
  (`/Game/Interface/W_Crosshair.ToggleHealFeedback` (`/Game/BluePrint/Data/BP_MenuManager.Crosshair` (`self.MenuManager`)) false))

(event `DecreaseComboValue`
  (bind _bp_weaponcomponent (`self.BP_WeaponComponent`))
  ;[1 0.4603 0.9097] Heal
  (`/Game/BluePrint/Entity/BP_WeaponComponent.Update Combo Level` _bp_weaponcomponent false (`/Game/BluePrint/Entity/BP_WeaponComponent.HealValuePerLoop` _bp_weaponcomponent) false))

(event `GainLife`
  ;[1 0.4603 0.9097] Heal
  (`FFMathBlueprintHelper.IncrementInt` (`self.PlayerLife`) 1)
  (`self.HealSuccess`)
  (`self.ClearHealBind`))

(event `ClearHealBind`
  ;[1 0.4603 0.9097] Heal
  (set `self.UsingLifeGain` false)
  (`KismetSystemLibrary.K2_ClearAndInvalidateTimerHandle` (stale `StartLifeGain` _returnvalue))
  (`KismetSystemLibrary.K2_ClearAndInvalidateTimerHandle` (stale `StartLifeGain` _returnvalue_2))
  (`/Game/Interface/W_Crosshair.ToggleHealFeedback` (`/Game/BluePrint/Data/BP_MenuManager.Crosshair` (`self.MenuManager`)) false))

(event `Make player invincible`
  (set `self.IsInvincible` true)
  (`KismetSystemLibrary.Delay` 3.0)
  (set `self.IsInvincible` false))

(event `GunShoot`
  ;[1 0.1649 0.1649] GameFeel
  (bind (_direction _addfov) (`Timeline|GunShootFOV` :!via `PlayFromStart`)
    (:`Update`
      (set `self.ShootFOV` _addfov))))

(event `GunHitEnemy`
  ;[1 0.1649 0.1649] GameFeel
)

(event `LaserStartCharge`
  (bind _t_laserfovincrease (`self.T_LaserFOVincrease`))
  ;[1 0.1649 0.1649] GameFeel
  (bind _returnvalue (`PlayerCameraManager.StartCameraShake` :`self` (`GameplayStatics.GetPlayerCameraManager` 0) :`ShakeClass` "/Game/CameraShake/CamShake_LaserCharge.CamShake_LaserCharge_C"))
  (set `self.CamShakeLaserCharge` _returnvalue)
  (`TimelineComponent.Stop` (`self.T_LaserFOVdecrease`))
  (`TimelineComponent.SetNewTime` _t_laserfovincrease (`self.CurrentLaserFOV`))
  (`TimelineComponent.SetPlayRate` _t_laserfovincrease (/ 1.0 1.5))
  (`TimelineComponent.SetPlayRate` (`self.T_LaserFOVincrease`) (/ 1.0 0.5))
  (bind (_direction _addfov _time) (`Timeline|T_LaserFOVincrease`)
    (:`Update`
      (set `self.CurrentLaserFOV` _time)
      (set `self.ShootFOV` (* _addfov 8.0))
      (set `PostProcessComponent.BlendWeight` _addfov (`self.LaserPostProcess`))
      (`KismetMaterialLibrary.SetScalarParameterValue` "/Game/Materials/PostPro/PostProPara.PostProPara" "LaserBlendWeight" _addfov))
    (:`Finished`
      (bind (_direction_2 _addfov_2) (`Timeline|LaserFOVstay` :!via `PlayFromStart`)
        (:`Update`
          (set `self.ShootFOV` (+ _addfov_2 8.0)))))))

(event `LaserStartShoot`
  (bind _returnvalue (`GameplayStatics.GetPlayerCameraManager` 0))
  ;[1 0.1649 0.1649] GameFeel
  (`PlayerCameraManager.StopCameraShake` _returnvalue (`self.CamShakeLaserCharge`) false)
  (bind _returnvalue_2 (`PlayerCameraManager.StartCameraShake` :`self` _returnvalue :`ShakeClass` "/Game/CameraShake/CamShake_LaserShoot.CamShake_LaserShoot_C"))
  (set `self.CamShakeLaser` _returnvalue_2)
  (bind (_direction _addfov) (`Timeline|T_LaserStart` :!via `PlayFromStart`)
    (:`Update`
      (set `self.ShootFOVNiveau` (* _addfov 8.0)))))

(event `LaserEndShoot`
  (bind _returnvalue (`GameplayStatics.GetPlayerCameraManager` 0))
  (bind _t_laserfovdecrease (`self.T_LaserFOVdecrease`))
  ;[1 0.1649 0.1649] GameFeel
  (`PlayerCameraManager.StopCameraShake` _returnvalue (`self.CamShakeLaserCharge`) false)
  (`PlayerCameraManager.StopCameraShake` _returnvalue (`self.CamShakeLaser`) false)
  (`TimelineComponent.Stop` (`self.T_LaserFOVincrease`))
  (`TimelineComponent.Stop` (`self.LaserFOVstay`))
  (`TimelineComponent.SetNewTime` _t_laserfovdecrease (`self.CurrentLaserFOV`))
  (`TimelineComponent.SetPlayRate` _t_laserfovdecrease (/ 1.0 0.5))
  (bind (_direction _addfov) (`Timeline|T_LaserFOVdecrease` :!via `Reverse`)
    (:`Update`
      (set `self.CurrentLaserFOV` _addfov)
      (set `self.ShootFOV` (* _addfov 8.0))
      (set `PostProcessComponent.BlendWeight` _addfov (`self.LaserPostProcess`))
      (`KismetMaterialLibrary.SetScalarParameterValue` "/Game/Materials/PostPro/PostProPara.PostProPara" "LaserBlendWeight" _addfov))))

(event `MinusOneChargeBar`
  ;[1 0.1649 0.1649] GameFeel
  (`PlayerCameraManager.StartCameraShake` :`self` (`GameplayStatics.GetPlayerCameraManager` 0) :`ShakeClass` "/Game/CameraShake/CamShake_LaserLevelDown.CamShake_LaserLevelDown_C")
  (bind (_direction _addfov) (`Timeline|Timeline` :!via `PlayFromStart`)
    (:`Update`
      (set `self.ShootFOVNiveau` _addfov))))

(event `HealStart`
  (bind _t_healfov (`self.T_HealFOV`))
  ;[1 0.1649 0.1649] GameFeel
  ;;[0.8334 0.2497 1] Heal stuff
  (bind _returnvalue (`PlayerCameraManager.StartCameraShake` :`self` (`GameplayStatics.GetPlayerCameraManager` 0) :`ShakeClass` "/Game/CameraShake/CamShake_HealingShake.CamShake_HealingShake_C"))
  (set `self.CamShakeHeal` _returnvalue)
  (`TimelineComponent.SetNewTime` _t_healfov (`self.CurrentHealingFOVtimeline`))
  (`TimelineComponent.SetPlayRate` _t_healfov (/ 1.0 2.0))
  (bind (_direction _addfov) (`Timeline|T_HealFOV`)
    (:`Update`
      (set `self.HealFOV` (* _addfov 16.0))
      (set `self.CurrentHealingFOVtimeline` (`KismetMathLibrary.Abs` _addfov)))))

(event `HealCancel`
  (bind _t_reversehealing (`self.T_ReverseHealing`))
  ;[1 0.1649 0.1649] GameFeel
  ;;[0.8334 0.2497 1] Heal stuff
  (`PlayerCameraManager.StopCameraShake` (`GameplayStatics.GetPlayerCameraManager` 0) (`self.CamShakeHeal`) false :!label _label_2)
  (`TimelineComponent.Stop` (`self.T_HealFOV`))
  (`TimelineComponent.SetNewTime` _t_reversehealing (`self.CurrentHealingFOVtimeline`))
  (`TimelineComponent.SetPlayRate` _t_reversehealing (/ 1.0 0.3))
  (bind (_direction _addfov) (`Timeline|T_ReverseHealing` :!via `Reverse`)
    (:`Update`
      (set `self.HealFOV` (* _addfov 16.0))
      (set `self.CurrentHealingFOVtimeline` (`KismetMathLibrary.Abs` _addfov)))))

(event `HealSuccess`
  ;[1 0.1649 0.1649] GameFeel
  ;;[0.8334 0.2497 1] Heal stuff
  (`PlayerCameraManager.StartCameraShake` :`self` (`GameplayStatics.GetPlayerCameraManager` 0) :`ShakeClass` "/Game/CameraShake/CamShake_HealedShake.CamShake_HealedShake_C")
  (goto _label_2))

(fn `ChangeStats`
  (params (Profil :type "/Game/BluePrint/Data/E_PlayerProfiles Enum" :default "NewEnumerator0"))
  (bind _output_get (set `self.PlayerRow` (make `DataTableRowHandle` "/Game/BluePrint/Data/DT_PlayerDataTable.DT_PlayerDataTable" (`KismetStringLibrary.Conv_StringToName` (`|GetEnumeratorNameAsString` Profil)))))
  (bind (_datatable _rowname) (break `DataTableRowHandle` _output_get))
  (bind _returnvalue (`|GetDataTableRow` _datatable _rowname)
    (:`then`
      (set `self.PlayerStats` _returnvalue))))

(fn `Die`
  (bind _menumanager (`self.MenuManager`))
  (`/Game/BluePrint/Data/BP_MenuManager.StopGame` _menumanager)
  (`/Game/BluePrint/Data/BP_MenuManager.ShowGameOver` _menumanager)
  (`AkGameplayStatics.PostEvent` "/Game/WwiseAudio/Events/Default_Work_Unit/behaviour/DEATH.DEATH"))

(fn `LoseLife`
  (params (IsLosingLife :type Boolean) (DamagePos :type "Vector Structure") (Enemy :type "Actor Object Reference"))
  (if (not (`self.IsInvincible`))
    (`FFMathBlueprintHelper.DecrementInt` (`self.PlayerLife`) 1)
    (`FFMathBlueprintHelper.ClampIntByRef` (`self.PlayerLife`) 0 (`self.PlayerMaxLife`))
    (if IsLosingLife
      (`self.Make player invincible`)
      (`self.StopLifeGain`)
      (`/Game/Interface/W_Crosshair.Take Damage` (`/Game/BluePrint/Data/BP_MenuManager.Crosshair` (`self.MenuManager`)) (0.5 0.5 0.0))
      (bind _returnvalue (`|CreateWidget` "/Game/Interface/W_HitWidget.W_HitWidget_C"))
      (set `/Game/Interface/W_HitWidget.Target` Enemy _returnvalue)
      (`UserWidget.AddToViewport` _returnvalue 0)
      (if (<= (`self.PlayerLife`) 0)
        (`self.Die`)))))

(fn `Music`
  (locals (CloseCount :type Integer))
  (bind _returnvalue (`FFEnemyControl.GetAllEnemies` (`self.EnemyControl`)))
  (for _array_element _returnvalue
    (bind _asbp_base_enemy (cast `/Game/BluePrint/Entity/Enemy/BP_BaseEnemy` _array_element))
    (if (< (`KismetMathLibrary.Vector_Distance` (`SceneComponent.K2_GetComponentLocation` (`Character.CapsuleComponent` _asbp_base_enemy)) (`SceneComponent.K2_GetComponentLocation` (`self.PlayerCol`))) (`self.M_EnemyDistPlayer`))
      (`/Engine/EditorBlueprintResources/StandardMacros.IncrementInt` (`local.CloseCount`))))
  (if (> (`local.CloseCount`) (`self.M_Phase4Count`))
    (`AkGameplayStatics.SetState` "/Game/WwiseAudio/States/Default_Work_Unit/Music/Music-Phase_3.Music-Phase_3")
    (`AkGameplayStatics.SetState` "/Game/WwiseAudio/States/Default_Work_Unit/Phase3_Loop/Phase3_Loop-Loop.Phase3_Loop-Loop")
    (elif (> (`local.CloseCount`) (`self.M_Phase3Count`))
      (`AkGameplayStatics.SetState` "/Game/WwiseAudio/States/Default_Work_Unit/Music/Music-Phase_3.Music-Phase_3")
      (`AkGameplayStatics.SetState` "/Game/WwiseAudio/States/Default_Work_Unit/Phase3_Loop/Phase3_Loop-Intro.Phase3_Loop-Intro")
      (elif (> (`local.CloseCount`) (`self.M_Phase2Count`))
        (`AkGameplayStatics.SetState` "/Game/WwiseAudio/States/Default_Work_Unit/Music/Music-Phase_2.Music-Phase_2")
        (else
          (`AkGameplayStatics.SetState` "/Game/WwiseAudio/States/Default_Work_Unit/Music/Music-Phase_1.Music-Phase_1"))))))

(fn `Speed Feed Back`
  (returns (FOV :type "Float (double-precision)"))
  (locals (LowerRange :type "Float (double-precision)" :default 20.0) (TopRange :type "Float (double-precision)" :default 150.0) (Smooth :type "Float (double-precision)"))
  (bind _returnvalue (`KismetMathLibrary.VSize` (`KismetMathLibrary.MakeVector` (.x (`FFMovementBehavior.CurVelocity` (`self.FFMovementBehavior`))) (.y (`FFMovementBehavior.CurVelocity` (`self.FFMovementBehavior`))))))
  (if (!= (`/Game/BluePrint/Entity/BP_MovementComponenet.Grounded` (`self.BP_MovementComponent`)) true)
    (return (`self.CurrentFOV`))
    (else
      (bind _returnvalue_2 (`FFBlueprintHelper.EvaluateCurve` "/Game/Curve/FC_FOVSpeedCurve.FC_FOVSpeedCurve" _returnvalue))
      (if (`/Game/BluePrint/Entity/BP_MovementComponenet.IsSliding` (`self.BP_MovementComponent`))
        (set `local.Smooth` 10.0)
        (else
          (set `local.Smooth` 1.0)))
      (bind _returnvalue_3 (`FFBlueprintHelper.SmoothValueByRef` (`self.CurrentFOV`) (`KismetMathLibrary.FClamp` _returnvalue_2 (`local.LowerRange`) (`local.TopRange`)) (`local.Smooth`) (`GameplayStatics.GetWorldDeltaSeconds`)))
      (`KismetMaterialLibrary.SetScalarParameterValue` "/Game/Materials/PostPro/PostProPara.PostProPara" "SpeedLineBlendWeight" (`KismetMathLibrary.MapRangeClamped` _returnvalue 840.0 1100.0 0.0 1.0))
      (return _returnvalue_3))))

(fn `UserConstructionScript`
  (`parent.UserConstructionScript`))
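; BP_Enemy is an enemy entity Blueprint that takes damage and reports which body part was hit.
; DamagePlace passes the incoming damage straight to LoseLife, with no scaling by body part.
; It then looks up the touched part's physical material in BodyPartsMap and prints the part name and damage as debug text.
; The event graph holds only disabled default events, and the construction script just calls its parent.
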(fn `DamagePlace`
  (params (TouchedPart :type "HitResult Structure") (Damages :type Integer))
  (`self.LoseLife` Damages)
  (`KismetSystemLibrary.PrintString` (`KismetStringLibrary.Concat_StrStr` "Hit enemy in" (`|GetEnumeratorNameAsString` (`BlueprintMapLibrary.Map_Find` (`self.BodyPartsMap`) (`.PhysMat` (`GameplayStatics.BreakHitResult` TouchedPart)))) " [-" (`KismetStringLibrary.Conv_IntToString` Damages) " hp]")))

(fn `UserConstructionScript`
  (`parent.UserConstructionScript`))
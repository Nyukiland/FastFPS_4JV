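; Split ground enemy Blueprint that extends a parent enemy, selecting the "Split" data row name and the BT_GroundSplit behavior tree on BeginPlay.
; While in the Attack state, a capsule hit on the player deals damage once, guarded by HitOnce, and stores the impact normal.
; On death it disables cube and capsule collision, then enables physics simulation and gravity on the capsule.
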(event `self.ReceiveBeginPlay`
  (set `self.EnemyRowName` "Split")
  (set `self.BehaviorTree` "/Game/BluePrint/Entity/Enemy/GroundEnemy/Split/BT_GroundSplit.BT_GroundSplit")
  (`parent.ReceiveBeginPlay`))

(event `self.StartState`
  ;[1 1 1] behavior tree
  (`parent.StartState`))

(event `self.TickState`
  ;[1 1 1] behavior tree
  (`parent.TickState`))

(event `self.Fail`
  ;[1 1 1] behavior tree
  (`parent.Fail`))

(event `self.CapsuleComponent.OnComponentHit`
  (params (HitComponent :type "PrimitiveComponent Object Reference") (OtherActor :type "Actor Object Reference") (OtherComp :type "PrimitiveComponent Object Reference") (NormalImpulse :type "Vector Structure") (Hit :type "HitResult Structure (by ref)"))
  (if (not (`self.HitOnce`))
    (switch `/Game/BluePrint/Entity/Enemy/GroundEnemy/Split/E_EnemyState` (`self.State`)
      (:`NewEnumerator2`
        (bind _asbp_player (cast `/Game/BluePrint/Entity/BP_Player` OtherActor))
        (`/Game/BluePrint/Entity/BP_Player.LoseLife` _asbp_player (`.Damage_8_D984C1F2427136DE6BE4799A6E4E808E` (break `/Game/BluePrint/Data/S_Enemy` (`self.controlVar`))))
        (set `self.NormalHit` (`.ImpactNormal` (`GameplayStatics.BreakHitResult` Hit)))
        (set `self.HitOnce` true)))))

(fn `Death`
  (bind _capsulecomponent (`self.CapsuleComponent`))
  (`parent.Death`)
  (`PrimitiveComponent.SetCollisionEnabled` (`self.Cube`) "NoCollision")
  (`PrimitiveComponent.SetCollisionEnabled` _capsulecomponent "NoCollision")
  (`PrimitiveComponent.SetSimulatePhysics` _capsulecomponent true)
  (`PrimitiveComponent.SetEnableGravity` _capsulecomponent true))

(fn `UserConstructionScript`)
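; Combined ground enemy that damages the player on a dashing hit and splits into a BP_SplitEnemy per stacked skeletal part on death.
; State changes drive the base and part animation blueprints.
; First damage starts a fuse: expiry kills it in an explosion that propels nearby split and combined enemies, while earlier death plays a melting sound.
; Dynamic materials show remaining life as heat and dissolve the body before destruction.
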(event `self.ReceiveBeginPlay`
  (set `self.EnemyRowName` "Combined")
  (set `self.BehaviorTree` "/Game/BluePrint/Entity/Enemy/GroundEnemy/BT_GroundCombined.BT_GroundCombined")
  (`parent.ReceiveBeginPlay`)
  (`KismetArrayLibrary.Array_Add` (`self.Split`) (`self.SkeletalMesh`))
  (`KismetArrayLibrary.Array_Add` (`self.Split`) (`self.SkeletalMesh1`))
  (`KismetArrayLibrary.Array_Add` (`self.Split`) (`self.SkeletalMesh2`))
  (bind _returnvalue (`PrimitiveComponent.CreateDynamicMaterialInstance` (`self.Mesh`) 0 "/Game/Materials/Monstre/M_Base_Marchant.M_Base_Marchant" "None"))
  (set `self.BaseMat` _returnvalue)
  (bind _returnvalue_2 (`PrimitiveComponent.CreateDynamicMaterialInstance` (`self.Mesh`) 1 "/Game/Materials/Monstre/M_Lights.M_Lights" "None"))
  (set `self.LightMat` _returnvalue_2)
  (`self.AddToPivotAndCollider` (`self.Box2`))
  (`self.AddToPivotAndCollider` (`self.SkeletalMesh`))
  (`self.AddToPivotAndCollider` (`self.SkeletalMesh1`))
  (`self.AddToPivotAndCollider` (`self.SkeletalMesh2`))
  (`self.AddToPivotAndCollider` (`self.Box`))
  (`self.AddToPivotAndCollider` (`self.Box1`)))

(event `self.ReceiveTick`
  (params (DeltaSeconds :type "Float (single-precision)"))
  (`parent.ReceiveTick` DeltaSeconds)
  (if (!= (`self.TimerSplit`) -1.0)
    (bind _returnvalue (`FFMathBlueprintHelper.IncrementFloat` (`self.TimerSplit`) DeltaSeconds))
    (if (> _returnvalue (`self.MaxTimerDeath`))
      (`/Engine/EditorBlueprintResources/StandardMacros.DoOnce` false
        (:`Completed`
          (`self.Death`))))))

(event `self.CapsuleComponent.OnComponentHit`
  (params (HitComponent :type "PrimitiveComponent Object Reference") (OtherActor :type "Actor Object Reference") (OtherComp :type "PrimitiveComponent Object Reference") (NormalImpulse :type "Vector Structure") (Hit :type "HitResult Structure (by ref)"))
  (if (not (`self.HitOnce`))
    (switch `/Game/BluePrint/Entity/Enemy/E_EnemyState` (`self.State`)
      (:`NewEnumerator2`
        (bind _asbp_player (cast `/Game/BluePrint/Entity/BP_Player` OtherActor))
        (`/Game/BluePrint/Entity/BP_Player.LoseLife` _asbp_player true (`SceneComponent.K2_GetComponentLocation` (`self.CapsuleComponent`)) OtherActor)
        (set `self.NormalHit` (`.ImpactNormal` (`GameplayStatics.BreakHitResult` Hit)))
        (set `self.HitOnce` true)))))

(event `self.StartState`
  (`parent.StartState`)
  (`|ExecutionSequence`
    (:`then_0`
      (set `self.randomStartPos` (`KismetMathLibrary.RandomFloatInRange` 0.0 1.5))
      (for _array_element (`self.Split`)
        (bind _asabp_ennemy_marchant (cast `/Game/FBX/Monstre/Splitting/ABP_EnnemyMarchant` (`SkeletalMeshComponent.GetAnimInstance` _array_element)))
        (switch `/Game/BluePrint/Entity/Enemy/E_EnemyState` (`self.State`)
          (:`NewEnumerator0`
            (set `/Game/FBX/Monstre/Splitting/ABP_EnnemyMarchant.Dashing` false _asabp_ennemy_marchant)
            (set `/Game/FBX/Monstre/Splitting/ABP_EnnemyMarchant.Walking` true _asabp_ennemy_marchant)
            (set `/Game/FBX/Monstre/Splitting/ABP_EnnemyMarchant.StartPos` (`self.randomStartPos`) _asabp_ennemy_marchant :!label _label))
          (:`NewEnumerator1`
            (set `/Game/FBX/Monstre/Splitting/ABP_EnnemyMarchant.Dashing` false _asabp_ennemy_marchant)
            (set `/Game/FBX/Monstre/Splitting/ABP_EnnemyMarchant.Walking` false _asabp_ennemy_marchant))
          (:`NewEnumerator2`
            (`AkGameplayStatics.PostEvent` "/Game/WwiseAudio/Events/Default_Work_Unit/Ennemy/ROBOT/Voice_Robot.Voice_Robot" self)
            (set `/Game/FBX/Monstre/Splitting/ABP_EnnemyMarchant.Dashing` true _asabp_ennemy_marchant)
            (set `/Game/FBX/Monstre/Splitting/ABP_EnnemyMarchant.Walking` false _asabp_ennemy_marchant)
            (goto _label)))))
    (:`then_1`
      (bind _asabp_base (cast `/Game/FBX/Monstre/Splitting/Base/ABP_Base` (`SkeletalMeshComponent.GetAnimInstance` (`self.Mesh`))))
      (switch `/Game/BluePrint/Entity/Enemy/E_EnemyState` (`self.State`)
        (:`NewEnumerator0`
          (set `/Game/FBX/Monstre/Splitting/Base/ABP_Base.IsWalk` true _asabp_base)
          (set `/Game/FBX/Monstre/Splitting/Base/ABP_Base.IsDash` false _asabp_base))
        (:`NewEnumerator1`
          (set `/Game/FBX/Monstre/Splitting/Base/ABP_Base.IsWalk` false _asabp_base)
          (set `/Game/FBX/Monstre/Splitting/Base/ABP_Base.IsDash` true _asabp_base))
        (:`NewEnumerator2`
          (set `/Game/FBX/Monstre/Splitting/Base/ABP_Base.IsWalk` false _asabp_base)
          (set `/Game/FBX/Monstre/Splitting/Base/ABP_Base.IsDash` true _asabp_base))))))

(fn `ChangeMatLifeColor`
  (`MaterialInstanceDynamic.SetScalarParameterValue` (`self.BaseMat`) "HeatDissolve" (`KismetMathLibrary.FClamp` (/ (`self.LifePoint`) (`self.MaxLife`)))))

(fn `DamagePlace`
  (params (TouchedPart :type "HitResult Structure") (Damage :type "Float (double-precision)") (Laser :type Boolean))
  (`parent.DamagePlace` TouchedPart Damage false)
  (bind _asabp_base (cast `/Game/FBX/Monstre/Splitting/Base/ABP_Base` (`SkeletalMeshComponent.GetAnimInstance` (`self.Mesh`))))
  (set `/Game/FBX/Monstre/Splitting/Base/ABP_Base.TakeDamage` true _asabp_base)
  (if (== (`self.TimerSplit`) -1.0)
    (set `self.TimerSplit` 0.0)))

(fn `Death`
  (locals (PropelZoneDist :type "Float (single-precision)" :default 300.0))
  (bind _returnvalue (`SceneComponent.K2_GetComponentLocation` (`self.CapsuleComponent`)))
  (`AkGameplayStatics.PostEvent` "/Game/WwiseAudio/Events/Default_Work_Unit/Ennemy/ROBOT/STOP_Timer.STOP_Timer" self)
  (bind _asabp_base (cast `/Game/FBX/Monstre/Splitting/Base/ABP_Base` (`SkeletalMeshComponent.GetAnimInstance` (`self.Mesh`))))
  (set `/Game/FBX/Monstre/Splitting/Base/ABP_Base.IsDead` true _asabp_base)
  (`NiagaraFunctionLibrary.SpawnSystemAtLocation` "/Game/VFX/smoke/VFX_SmokeExplosion.VFX_SmokeExplosion" (`SceneComponent.K2_GetComponentLocation` (`self.SkeletalMesh1`)))
  (for (_array_element _array_index) (`self.Split`)
    (`PrimitiveComponent.SetCollisionEnabled` _array_element "NoCollision")
    (`ActorComponent.Deactivate` _array_element)
    (`SceneComponent.SetVisibility` _array_element false false)
    (bind (_returnvalue_location _returnvalue_rotation) (`KismetMathLibrary.BreakTransform` (`SceneComponent.K2_GetComponentToWorld` _array_element)))
    (`|SpawnActorFromClass` "/Game/BluePrint/Entity/Enemy/Split/BP_SplitEnemy.BP_SplitEnemy_C" (`KismetMathLibrary.MakeTransform` (+ _returnvalue_location (`KismetMathLibrary.MakeVector` (`KismetMathLibrary.FClamp` (* (`KismetMathLibrary.RandomFloat`) 100.0) 0.0 300.0) (`KismetMathLibrary.FClamp` (* (`KismetMathLibrary.RandomFloat`) 100.0) 0.0 300.0) (* 75.0 (+ _array_index 1)))) _returnvalue_rotation) "AdjustIfPossibleButDontSpawnIfColliding" "MultiplyWithRoot" null null))
  (if (>= (`self.TimerSplit`) (`self.MaxTimerDeath`))
    (`AkGameplayStatics.PostEvent` "/Game/WwiseAudio/Events/Default_Work_Unit/Ennemy/ROBOT/EXPLODIN.EXPLODIN" self)
    (`NiagaraFunctionLibrary.SpawnSystemAtLocation` "/Game/VFX/smoke/VFX_Explosion.VFX_Explosion" (`SceneComponent.K2_GetComponentLocation` (`self.CapsuleComponent`)))
    (bind _outactors (`KismetSystemLibrary.SphereOverlapActors` _returnvalue (`local.PropelZoneDist`) (`|MakeArray` "ObjectTypeQuery8" "ObjectTypeQuery3" :!type "EObjectTypeQuery Enum") "/Game/BluePrint/Entity/Enemy/BP_BaseEnemy.BP_BaseEnemy_C"))
    (for _array_element_2 _outactors
      (bind _returnvalue_2 (`GameplayStatics.GetObjectClass` _array_element_2))
      (if (and (or (== _returnvalue_2 "/Game/BluePrint/Entity/Enemy/Split/BP_SplitEnemy.BP_SplitEnemy_C") (== _returnvalue_2 "BP_CombinedEnemy_C")) (!= _array_element_2 self))
        (bind _asbp_base_enemy (cast `/Game/BluePrint/Entity/Enemy/BP_BaseEnemy` _array_element_2))
        (`self.PropelEnemy` _asbp_base_enemy _returnvalue (`local.PropelZoneDist`))))
    (else
      (`AkGameplayStatics.PostEvent` "/Game/WwiseAudio/Events/Default_Work_Unit/Ennemy/ROBOT/MELTING.MELTING" self)))
  (`parent.Death`))

(fn `Death Delay`
  (params (deltaTime :type "Float (double-precision)"))
  (bind _timerdeath (`self.TimerDeath`))
  (if (!= _timerdeath -1.0)
    (bind _returnvalue (`FFMathBlueprintHelper.IncrementFloat` _timerdeath deltaTime))
    (bind _returnvalue_2 (`KismetMathLibrary.Abs` (- (`KismetMathLibrary.FClamp` (/ _returnvalue (`.EnemyDeathSpeed_51_25410B914FA95D940827A6A4B502FA4F` (break `/Game/BluePrint/Data/S_Enemy` (`self.controlVar`))))) 1.0)))
    (`MaterialInstanceDynamic.SetScalarParameterValue` (`self.BaseMat`) "DeathDissolve" _returnvalue_2)
    (`MaterialInstanceDynamic.SetScalarParameterValue` (`self.LightMat`) "DeathDissolve" _returnvalue_2)
    (if (> (`self.TimerDeath`) (`.EnemyDeathSpeed_51_25410B914FA95D940827A6A4B502FA4F` (break `/Game/BluePrint/Data/S_Enemy` (`self.controlVar`))))
      (`self.K2_DestroyActor` self))))

(fn `UserConstructionScript`
  (`parent.UserConstructionScript`))
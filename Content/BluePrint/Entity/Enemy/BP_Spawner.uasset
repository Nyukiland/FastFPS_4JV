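; BP_Spawner is a stationary, destructible enemy that spawns combined enemies during waves, plus flying enemies overhead shortly after it starts.
; It reads stats from a data table, registers with EnemyControl and uses its wave info to time and cap spawns, opening its animated door.
; Laser damage is reduced, and death during a wave credits its share of the wave's enemy count as spawned.
; Dynamic materials show health, death dissolve and an idle pulse alongside Wwise audio.
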(event `self.ReceiveBeginPlay`
  (bind _returnvalue (`|GetDataTableRow` "/Game/BluePrint/Data/DT_EnemyDataTable.DT_EnemyDataTable" (`self.EnemyRowName`))
    (:`then`
      (bind _output_get (set `self.controlVar` _returnvalue))
      (bind _output_get_2 (set `self.MaxLife` (`.Life_6_E7CAA32E4602CF532D46529ECF629B4E` (break `/Game/BluePrint/Data/S_Enemy` _output_get))))
      (set `self.LifePoint` _output_get_2)
      (bind _returnvalue_2 (`PrimitiveComponent.CreateDynamicMaterialInstance` (`self.Mesh`) 0 "/Game/Materials/Monstre/M_Spawner.M_Spawner" "None"))
      (set `self.Mat` _returnvalue_2)
      (bind _returnvalue_3 (`PrimitiveComponent.CreateDynamicMaterialInstance` (`self.Mesh`) 1 "/Game/Materials/Monstre/M_Lights.M_Lights" "None"))
      (set `self.Light` _returnvalue_3)
      (bind _returnvalue_4 (`PrimitiveComponent.CreateDynamicMaterialInstance` (`self.CharacterMesh1`) 0 "/Game/Materials/MA_Seethrough.MA_Seethrough" "None"))
      (set `self.Pulse` _returnvalue_4)
      (`CharacterMovementComponent.DisableMovement` (`self.CharacterMovement`))
      (bind _returnvalue_5 (`FFEnemyControl.GetEnemyControl` self))
      (bind _output_get_3 (set `self.EnemyControl` _returnvalue_5))
      (`FFEnemyControl.RegisterEnemySpawned` _output_get_3 self)
      (bind _returnvalue_6 (`FFEnemyControl.GetCurrentWaveInfo` (`self.EnemyControl`)))
      (set `self.CurWaveInfo` _returnvalue_6)
      (set `self.Timer` (`KismetMathLibrary.RandomFloat`))
      (`self.WaitForSpawnFlying`))))

(event `WaitForSpawnFlying`
  (`KismetSystemLibrary.DelayUntilNextTick`)
  (`KismetSystemLibrary.DelayUntilNextTick`)
  (`KismetSystemLibrary.DelayUntilNextTick`)
  (for _ (range 1 (+ (`.FlyingOnSpawner` (break `WaveSetUp` (`self.CurWaveInfo`))) 1))
    (bind _returnvalue (`FFMathBlueprintHelper.RandomVector` 200.0))
    (bind _returnvalue_2 (`|SpawnActorFromClass` "/Game/BluePrint/Entity/Enemy/FlyingEnemy/BP_FlyingEnemy.BP_FlyingEnemy_C" (`KismetMathLibrary.MakeTransform` (+ _returnvalue (`SceneComponent.K2_GetComponentLocation` (`self.Mesh`)) (0.0 0.0 800.0))) "AdjustIfPossibleButAlwaysSpawn" "MultiplyWithRoot" null null))
    (set `/Game/BluePrint/Entity/Enemy/FlyingEnemy/BP_FlyingEnemy.Spawner` self _returnvalue_2)))

(event `self.ReceiveTick`
  (params (DeltaSeconds :type "Float (single-precision)"))
  (`parent.ReceiveTick` DeltaSeconds)
  (`self.Spawn` DeltaSeconds)
  (`self.WaveSoundAndFeedback` DeltaSeconds))

(fn `ChangeMatLifeColor`
  (`MaterialInstanceDynamic.SetScalarParameterValue` (`self.Mat`) "HeatDissolve" (`KismetMathLibrary.FClamp` (/ (`self.LifePoint`) (`self.MaxLife`)))))

(fn `DamagePlace`
  (params (TouchedPart :type "HitResult Structure") (Damage :type "Float (double-precision)") (Laser :type Boolean))
  (returns (TouchedBodyPart :type "/Game/BluePrint/Data/E_BodyParts Enum"))
  (locals (DamageLocal :type "Float (double-precision)" :default 0.0))
  (set `local.DamageLocal` Damage)
  (if Laser
    (set `local.DamageLocal` (/ (`local.DamageLocal`) 10.0)))
  (bind _touchedbodypart (`parent.DamagePlace` TouchedPart (`local.DamageLocal`) Laser))
  (return _touchedbodypart))

(fn `Death`
  (bind _enemycontrol (`self.EnemyControl`))
  (bind (_enemycount _flyingonspawner _spawnercount) (break `WaveSetUp` (`self.CurWaveInfo`)))
  (bind _enemyspawned (`FFEnemyControl.EnemySpawned` _enemycontrol))
  (`parent.Death`)
  (if (and (`|EnumEquality` (`FFEnemyControl.WaveState` _enemycontrol) "InWave") (< _enemyspawned _enemycount))
    (`FFMathBlueprintHelper.IncrementInt` _enemyspawned (/ _enemycount _spawnercount))))

(fn `Death Delay`
  (params (deltaTime :type "Float (double-precision)"))
  (bind _timerdeath (`self.TimerDeath`))
  (if (!= _timerdeath -1.0)
    (bind _returnvalue (`FFMathBlueprintHelper.IncrementFloat` _timerdeath deltaTime))
    (bind _returnvalue_2 (`KismetMathLibrary.Abs` (- (`KismetMathLibrary.FClamp` (/ _returnvalue (`.EnemyDeathSpeed_51_25410B914FA95D940827A6A4B502FA4F` (break `/Game/BluePrint/Data/S_Enemy` (`self.controlVar`))))) 1.0)))
    (`MaterialInstanceDynamic.SetScalarParameterValue` (`self.Mat`) "DeathDissolve" _returnvalue_2)
    (`MaterialInstanceDynamic.SetScalarParameterValue` (`self.Light`) "DeathDissolve" _returnvalue_2)
    (if (> (`self.TimerDeath`) (`.EnemyDeathSpeed_51_25410B914FA95D940827A6A4B502FA4F` (break `/Game/BluePrint/Data/S_Enemy` (`self.controlVar`))))
      (`self.K2_DestroyActor` self))))

(fn `GetCombinedEnemyCount`
  (returns (Count :type Integer))
  (locals (CountVar :type Integer :default 0))
  (for _array_element (`FFEnemyControl.EnemiesArray` (`self.EnemyControl`))
    (cast `/Game/BluePrint/Entity/Enemy/GroundEnemy/BP_CombinedEnemy` _array_element)
    (`/Engine/EditorBlueprintResources/StandardMacros.IncrementInt` (`local.CountVar`)))
  (return (`local.CountVar`)))

(fn `Spawn`
  (params (DelatTime :type "Float (single-precision)"))
  (bind (_enemycount _flyingonspawner _spawnercount _enemyatthesametime _timespawn) (break `WaveSetUp` (`self.CurWaveInfo`)))
  (bind _returnvalue (`FFMathBlueprintHelper.IncrementFloat` (`self.Timer`) DelatTime))
  (if (> _returnvalue _timespawn)
    (set `self.Timer` 0.0)
    (bind _count (`self.GetCombinedEnemyCount`))
    (if (and (< _count _enemyatthesametime) (< (`FFEnemyControl.EnemySpawned` (`self.EnemyControl`)) _enemycount))
      (`|SpawnActorFromClass` "/Game/BluePrint/Entity/Enemy/GroundEnemy/BP_CombinedEnemy.BP_CombinedEnemy_C" (`SceneComponent.K2_GetComponentToWorld` (`self.CapsuleComponent`)) "AdjustIfPossibleButAlwaysSpawn" "MultiplyWithRoot" null null)
      (`AkGameplayStatics.PostEvent` "/Game/WwiseAudio/Events/Default_Work_Unit/Spawners/Spawners_Open.Spawners_Open" self)
      (bind _asabp_spawner (cast `/Game/FBX/Spawner/ABP_Spawner` (`SkeletalMeshComponent.GetAnimInstance` (`self.Mesh`))))
      (set `/Game/FBX/Spawner/ABP_Spawner.DoorOpen` true _asabp_spawner))))

(fn `UserConstructionScript`
  (`parent.UserConstructionScript`))

(fn `WaveSoundAndFeedback`
  (params (deltaTime :type "Float (double-precision)"))
  (`|ExecutionSequence`
    (:`then_0`
      (if (== (`self.TimerSound`) 0.0)
        (`AkGameplayStatics.PostEvent` "/Game/WwiseAudio/Events/Default_Work_Unit/Spawners/Spawners_Idle.Spawners_Idle" self)))
    (:`then_1`
      (bind _returnvalue (`FFMathBlueprintHelper.IncrementFloat` (`self.TimerSound`) deltaTime))
      (`MaterialInstanceDynamic.SetScalarParameterValue` (`self.Pulse`) "Value" (`KismetMathLibrary.Abs` (- (`KismetMathLibrary.Abs` (* (- (`KismetMathLibrary.FClamp` _returnvalue 0.0 2.0) 1.0) 1.0)) 1.0)))
      (if (> (`self.TimerSound`) 5.0)
        (set `self.TimerSound` 0.0)))))
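; BP_EnemyGround is a robot ground enemy that chases the player and deals melee-range damage.
; A looping Move event runs AI MoveTo toward the player, stops after a timer, damages the player if within range, then waits and repeats.
; BeginPlay creates dynamic life-lerp materials for its meshes.
; Wwise events voice idle, attack and death, while states track robots being alive, switching to dead when the enemy manager's list is empty.
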(event `self.ReceiveBeginPlay`
  (`parent.ReceiveBeginPlay`)
  (bind _returnvalue (`PrimitiveComponent.CreateDynamicMaterialInstance` (`self.Cylinder`) 0 "/Game/Materials/MA_LifeLerp.MA_LifeLerp" "None"))
  (`KismetArrayLibrary.Array_Add` (`self.MaterialsInstanced`) _returnvalue)
  (bind _returnvalue_2 (`PrimitiveComponent.CreateDynamicMaterialInstance` (`self.Sphere`) 0 "/Game/Materials/MA_LifeLerp.MA_LifeLerp" "None"))
  (`KismetArrayLibrary.Array_Add` (`self.MaterialsInstanced`) _returnvalue_2)
  (`self.Move`)
  (`AkGameplayStatics.SetState` "/Game/WwiseAudio/States/Default_Work_Unit/Robot_life/Robot_life-alive.Robot_life-alive")
  (`AkGameplayStatics.PostEvent` "/Game/WwiseAudio/Events/Default_Work_Unit/Ennemy/ROBOT/iddle_robot.iddle_robot" self))

(event `Move`
  (`SkeletalMeshComponent.PlayAnimation` (`self.Mesh`) "/Game/Import/Enemy/MarchantProto_Anim.MarchantProto_Anim" true)
  (`|AIMoveTo` self (`SceneComponent.K2_GetComponentLocation` (`/Game/BluePrint/Entity/BP_Player.PlayerCol` (`self.Player`))) null
    (:`then`
      (`KismetSystemLibrary.Delay` (`self.TimerMoveMax`))
      (`MovementComponent.StopMovementImmediately` (`self.CharacterMovement`))
      (`SkeletalMeshComponent.PlayAnimation` (`self.Mesh`) null false)
      (if (< (`KismetMathLibrary.Vector_Distance` (`SceneComponent.K2_GetComponentLocation` (`/Game/BluePrint/Entity/BP_Player.PlayerCol` (`self.Player`))) (`SceneComponent.K2_GetComponentLocation` (`self.CapsuleComponent`))) (`self.Dist Damage`))
        (`AkGameplayStatics.PostEvent` "/Game/WwiseAudio/Events/Default_Work_Unit/Ennemy/ROBOT/Voice_Robot.Voice_Robot" self)
        (`/Game/BluePrint/Entity/BP_Player.LoseLife` (`self.Player`) (`self.Damage`)))
      (`KismetSystemLibrary.Delay` (`self.TimerWait`))
      (`self.Move`))))

(event `self.ReceiveTick`
  (params (DeltaSeconds :type "Float (single-precision)"))
  (`parent.ReceiveTick` DeltaSeconds))

(fn `Death`
  (`parent.Death`)
  (`AkGameplayStatics.PostEvent` "/Game/WwiseAudio/Events/Default_Work_Unit/Ennemy/ROBOT/Death_Robot.Death_Robot" self)
  (bind _returnvalue (`FFEnemyManager.GetEnemyManager` self))
  (bind _returnvalue_2 (`FFEnemyManager.GetAllEnemies` _returnvalue))
  (if (== (`KismetArrayLibrary.Array_Length` _returnvalue_2) 0)
    (`AkGameplayStatics.SetState` "/Game/WwiseAudio/States/Default_Work_Unit/Robot_life/Robot_life-dead.Robot_life-dead")))

(fn `UserConstructionScript`
  (`parent.UserConstructionScript`))
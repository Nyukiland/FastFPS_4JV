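; Split enemy child Blueprint, a ground robot that runs BT_GroundSplit and dashes to damage the player.
; State changes drive the animation Blueprint's walk and dash flags, with a voice on attack; a capsule hit while attacking costs the player life, gated by HitOnce.
; Damage flags laser or gun hit reactions.
; Dynamic materials show remaining life through HeatDissolve and fade body and lights through DeathDissolve before the actor is destroyed.
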(event `self.ReceiveBeginPlay`
  (set `self.EnemyRowName` "Split")
  (set `self.BehaviorTree` "/Game/BluePrint/Entity/Enemy/Split/BT_GroundSplit.BT_GroundSplit")
  (`parent.ReceiveBeginPlay`)
  (bind _returnvalue (`PrimitiveComponent.CreateDynamicMaterialInstance` (`self.Mesh`) 0 "/Game/Materials/Monstre/M_Marchant.M_Marchant" "None"))
  (set `self.MatMarchand` _returnvalue)
  (bind _returnvalue_2 (`PrimitiveComponent.CreateDynamicMaterialInstance` (`self.Mesh`) 1 "/Game/Materials/Monstre/M_Lights.M_Lights" "None"))
  (set `self.Light` _returnvalue_2)
  (bind _asabp_ennemy_marchant (cast `/Game/FBX/Monstre/Splitting/ABP_EnnemyMarchant` (`SkeletalMeshComponent.GetAnimInstance` (`self.Mesh`))))
  (set `self.AnimBP` _asabp_ennemy_marchant)
  (`self.AddToPivotAndCollider` (`self.Box`))
  (`self.AddToPivotAndCollider` (`self.Box1`))
  (`self.AddToPivotAndCollider` (`self.Box2`)))

(event `self.StartState`
  (bind _animbp (`self.AnimBP`))
  (bind _animbp_2 (`self.AnimBP`))
  (bind _animbp_3 (`self.AnimBP`))
  (`parent.StartState`)
  (switch `/Game/BluePrint/Entity/Enemy/E_EnemyState` (`self.State`)
    (:`NewEnumerator0`
      (set `/Game/FBX/Monstre/Splitting/ABP_EnnemyMarchant.Dashing` false _animbp_2)
      (set `/Game/FBX/Monstre/Splitting/ABP_EnnemyMarchant.Walking` true _animbp_2))
    (:`NewEnumerator1`
      (set `/Game/FBX/Monstre/Splitting/ABP_EnnemyMarchant.Dashing` false _animbp_3)
      (set `/Game/FBX/Monstre/Splitting/ABP_EnnemyMarchant.Walking` false _animbp_3))
    (:`NewEnumerator2`
      (`AkGameplayStatics.PostEvent` "/Game/WwiseAudio/Events/Default_Work_Unit/Ennemy/ROBOT/Voice_Robot.Voice_Robot" self)
      (set `/Game/FBX/Monstre/Splitting/ABP_EnnemyMarchant.Dashing` true _animbp)
      (set `/Game/FBX/Monstre/Splitting/ABP_EnnemyMarchant.Walking` false _animbp))))

(event `self.CapsuleComponent.OnComponentHit`
  (params (HitComponent :type "PrimitiveComponent Object Reference") (OtherActor :type "Actor Object Reference") (OtherComp :type "PrimitiveComponent Object Reference") (NormalImpulse :type "Vector Structure") (Hit :type "HitResult Structure (by ref)"))
  (if (not (`self.HitOnce`))
    (switch `/Game/BluePrint/Entity/Enemy/E_EnemyState` (`self.State`)
      (:`NewEnumerator2`
        (bind _asbp_player (cast `/Game/BluePrint/Entity/BP_Player` OtherActor))
        (`/Game/BluePrint/Entity/BP_Player.LoseLife` _asbp_player true (`SceneComponent.K2_GetComponentLocation` (`self.CapsuleComponent`)) OtherActor)
        (set `self.NormalHit` (`.ImpactNormal` (`GameplayStatics.BreakHitResult` Hit)))
        (set `self.HitOnce` true)))))

(event `self.ReceiveTick`
  (params (DeltaSeconds :type "Float (single-precision)"))
  (`parent.ReceiveTick` DeltaSeconds))

(fn `ChangeMatLifeColor`
  (`MaterialInstanceDynamic.SetScalarParameterValue` (`self.MatMarchand`) "HeatDissolve" (`KismetMathLibrary.FClamp` (/ (`self.LifePoint`) (`self.MaxLife`)))))

(fn `DamagePlace`
  (params (TouchedPart :type "HitResult Structure") (Damage :type "Float (double-precision)") (Laser :type Boolean))
  (bind _animbp (`self.AnimBP`))
  (`parent.DamagePlace` TouchedPart Damage false)
  (if Laser
    (set `/Game/FBX/Monstre/Splitting/ABP_EnnemyMarchant.HitLaser` true _animbp)
    (else
      (set `/Game/FBX/Monstre/Splitting/ABP_EnnemyMarchant.HitGun` true _animbp))))

(fn `Death`
  (`parent.Death`)
  (set `/Game/FBX/Monstre/Splitting/ABP_EnnemyMarchant.Dead` true (`self.AnimBP`)))

(fn `Death Delay`
  (params (deltaTime :type "Float (double-precision)"))
  (bind _timerdeath (`self.TimerDeath`))
  (if (!= _timerdeath -1.0)
    (bind _returnvalue (`FFMathBlueprintHelper.IncrementFloat` _timerdeath deltaTime))
    (bind _returnvalue_2 (`KismetMathLibrary.Abs` (- (`KismetMathLibrary.FClamp` (/ _returnvalue (`.EnemyDeathSpeed_51_25410B914FA95D940827A6A4B502FA4F` (break `/Game/BluePrint/Data/S_Enemy` (`self.controlVar`))))) 1.0)))
    (`MaterialInstanceDynamic.SetScalarParameterValue` (`self.MatMarchand`) "DeathDissolve" _returnvalue_2)
    (`MaterialInstanceDynamic.SetScalarParameterValue` (`self.Light`) "DeathDissolve" _returnvalue_2)
    (if (> (`self.TimerDeath`) (`.EnemyDeathSpeed_51_25410B914FA95D940827A6A4B502FA4F` (break `/Game/BluePrint/Data/S_Enemy` (`self.controlVar`))))
      (`self.K2_DestroyActor` self))))

(fn `UserConstructionScript`)
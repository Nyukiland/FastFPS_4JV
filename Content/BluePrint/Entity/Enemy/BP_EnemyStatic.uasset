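; BP_EnemyStatic is a stationary enemy that shows its life through its material color.
; BeginPlay loads life from the enemy data table, puts dynamic life-lerp materials on Sphere and Cube, registers with the enemy control and disables movement.
; Tick calls ChangeMatLifeColor to update the color.
; Death notifies the enemy control, spawns a particle system at the capsule and resets the death timer.
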(event `self.ReceiveBeginPlay`
  (bind _returnvalue (`|GetDataTableRow` "/Game/BluePrint/Data/DT_EnemyDataTable.DT_EnemyDataTable" (`self.EnemyRowName`))
    (:`then`
      (bind _output_get (set `self.controlVar` _returnvalue))
      (bind _output_get_2 (set `self.MaxLife` (`.Life_6_E7CAA32E4602CF532D46529ECF629B4E` (break `/Game/BluePrint/Data/S_Enemy` _output_get))))
      (set `self.LifePoint` _output_get_2)
      (bind _returnvalue_2 (`PrimitiveComponent.CreateDynamicMaterialInstance` (`self.Sphere`) 0 "/Game/Materials/MA_LifeLerp.MA_LifeLerp" "None"))
      (`KismetArrayLibrary.Array_Add` (`self.MaterialsInstanced`) _returnvalue_2)
      (bind _returnvalue_3 (`PrimitiveComponent.CreateDynamicMaterialInstance` (`self.Cube`) 0 "/Game/Materials/MA_LifeLerp.MA_LifeLerp" "None"))
      (`KismetArrayLibrary.Array_Add` (`self.MaterialsInstanced`) _returnvalue_3)
      (bind _returnvalue_4 (`FFEnemyControl.GetEnemyControl` self))
      (`FFEnemyControl.RegisterEnemySpawned` _returnvalue_4 self)
      (`CharacterMovementComponent.DisableMovement` (`self.CharacterMovement`)))))

(event `self.ReceiveTick`
  (params (DeltaSeconds :type "Float (single-precision)"))
  (`parent.ReceiveTick` DeltaSeconds)
  (`self.ChangeMatLifeColor`))

(fn `Death`
  (bind _returnvalue (`FFEnemyControl.GetEnemyControl` self))
  (`FFEnemyControl.EnemyDied` _returnvalue self)
  (`NiagaraFunctionLibrary.SpawnSystemAtLocation` null (`SceneComponent.K2_GetComponentLocation` (`self.CapsuleComponent`)))
  (set `self.TimerDeath` 0.0))

(fn `UserConstructionScript`
  (`parent.UserConstructionScript`))
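; Flying enemy that moves in timed bursts toward a point above the player and shoots projectiles at them.
; Each tick it turns to face the player and, during a burst, sets the Sphere's physics velocity toward a randomly offset target, scaled by a speed curve.
; When a burst ends, a DoOnce fires a BP_EnemyProjectile if the player is within range, pauses, then rerolls the offset for the next burst.
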(event `self.ReceiveBeginPlay`
  (`parent.ReceiveBeginPlay`)
  (bind _returnvalue (`PrimitiveComponent.CreateDynamicMaterialInstance` (`self.Sphere`) 0 "/Game/Materials/MA_LifeLerp.MA_LifeLerp" "None"))
  (`KismetArrayLibrary.Array_Add` (`self.MaterialsInstanced`) _returnvalue)
  (`SkeletalMeshComponent.PlayAnimation` (`self.Mesh`) "/Game/Import/Enemy/VolantProto_Anim.VolantProto_Anim" true)
  (`self.GetRandomOffset`))

(event `self.ReceiveTick`
  (params (DeltaSeconds :type "Float (single-precision)"))
  (`parent.ReceiveTick` DeltaSeconds)
  (`self.RotateToLookAt`)
  (bind _returnvalue (`FFMathBlueprintHelper.IncrementFloat` (`self.TimerMovement`) DeltaSeconds))
  (if (< _returnvalue (`self.TimeMaxMovement`))
    (`|ExecutionSequence`
      (:`then_0`
        (`self.Move`))
      (:`then_1`
        (goto _label :!via `Reset`)))
    (else
      (`/Engine/EditorBlueprintResources/StandardMacros.DoOnce` false :!label _label
        (:`Completed`
          (if (`self.Is Player Near Enemy`)
            (`self.Shoot`)
            (`KismetSystemLibrary.Delay` (`self.TimeWaitMovement`))
            (else
              (`KismetSystemLibrary.Delay` 0.2)))
          (set `self.TimerMovement` 0.0)
          (`self.GetRandomOffset`))))))

(fn `GetRandomOffset`
  (bind _returnvalue (`FFMathBlueprintHelper.RandomPointInCircle` (`self.RandomCircle`)))
  (set `self.RandomDir` (+ (* (0.0 0.0 1.0) (`KismetMathLibrary.BreakVector2D` _returnvalue)) (* (`SceneComponent.GetRightVector` (`self.CapsuleComponent`)) (`.Y` (`KismetMathLibrary.BreakVector2D` _returnvalue))))))

(fn `Is Player Near Enemy`
  (returns (IsNearEnemy :type Boolean))
  (return (< (`KismetMathLibrary.Vector_Distance` (`SceneComponent.K2_GetComponentLocation` (`self.CapsuleComponent`)) (`SceneComponent.K2_GetComponentLocation` (`/Game/BluePrint/Entity/BP_Player.PlayerCol` (`self.Player`)))) (`self.DistWithPlayer`))))

(fn `Move`
  (`PrimitiveComponent.SetPhysicsLinearVelocity` (`self.Sphere`) (* (`KismetMathLibrary.Normal` (- (+ (`SceneComponent.K2_GetComponentLocation` (`/Game/BluePrint/Entity/BP_Player.PlayerCol` (`self.Player`))) (`self.RandomDir`) (0.0 0.0 250.0)) (`SceneComponent.K2_GetComponentLocation` (`self.Sphere`)))) (`self.MovementSpeed`) (`CurveFloat.GetFloatValue` (`self.CurveMovement`) (`KismetMathLibrary.FClamp` (/ (`self.TimerMovement`) (`self.TimeMaxMovement`))))) false "None"))

(fn `RotateToLookAt`
  (bind _capsulecomponent (`self.CapsuleComponent`))
  (`SceneComponent.K2_SetWorldRotation` _capsulecomponent (`KismetMathLibrary.FindLookAtRotation` (`SceneComponent.K2_GetComponentLocation` _capsulecomponent) (`SceneComponent.K2_GetComponentLocation` (`/Game/BluePrint/Entity/BP_Player.PlayerCol` (`self.Player`)))) false false))

(fn `Shoot`
  (locals (distSpawn :type "Float (double-precision)" :default 100.0))
  (bind (_returnvalue_location _returnvalue_rotation _returnvalue_scale) (`KismetMathLibrary.BreakTransform` (`SceneComponent.K2_GetComponentToWorld` (`self.CapsuleComponent`))))
  (bind _returnvalue (`|SpawnActorFromClass` "/Game/BluePrint/Entity/Enemy/BP_EnemyProjectile.BP_EnemyProjectile_C" (`KismetMathLibrary.MakeTransform` (+ _returnvalue_location (* (`KismetMathLibrary.Normal` (- (`SceneComponent.K2_GetComponentLocation` (`/Game/BluePrint/Entity/BP_Player.PlayerCol` (`self.Player`))) (`SceneComponent.K2_GetComponentLocation` (`self.Sphere`)))) (`local.distSpawn`))) _returnvalue_rotation _returnvalue_scale) "AlwaysSpawn" "MultiplyWithRoot" null null))
  (`/Engine/EditorBlueprintResources/StandardMacros.IsValid` _returnvalue
    (:`Is Valid`
      (`/Game/BluePrint/Entity/Enemy/BP_EnemyProjectile.SetUpProjectile` _returnvalue (`KismetMathLibrary.Normal` (- (`SceneComponent.K2_GetComponentLocation` (`/Game/BluePrint/Entity/BP_Player.PlayerCol` (`self.Player`))) (`SceneComponent.K2_GetComponentLocation` (`self.Sphere`)))) (`self.Damage`)))))

(fn `UserConstructionScript`
  (`parent.UserConstructionScript`))
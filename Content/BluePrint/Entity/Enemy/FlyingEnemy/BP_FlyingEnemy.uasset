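; Flying enemy that runs the BT_Flying behavior tree and damages the player when its capsule hits them during an attack.
; CharacterMovement is off; helpers set hover height relative to the player and hand out cached NavMesh path points.
; Tick turns the pivot along its movement in Pursuit or Attack, otherwise toward the player.
; Damage and death set Anim Blueprint flags, while dynamic materials show remaining life and dissolve the body before destruction.
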(event `self.ReceiveBeginPlay`
  (set `self.EnemyRowName` "Flying")
  (set `self.BehaviorTree` "/Game/BluePrint/Entity/Enemy/FlyingEnemy/BT_Flying.BT_Flying")
  (`parent.ReceiveBeginPlay`)
  (`ActorComponent.Deactivate` (`self.CharacterMovement`))
  (set `self.prevPos` (`SceneComponent.K2_GetComponentLocation` (`self.CapsuleComponent`)))
  (bind _returnvalue (`PrimitiveComponent.CreateDynamicMaterialInstance` (`self.Mesh`) 0 "/Game/Materials/Monstre/M_Volant.M_Volant" "None"))
  (set `self.MatVolant` _returnvalue)
  (bind _returnvalue_2 (`PrimitiveComponent.CreateDynamicMaterialInstance` (`self.Mesh`) 1 "/Game/Materials/Monstre/M_Lights.M_Lights" "None"))
  (set `self.Mat light` _returnvalue_2)
  (bind _asabp_volant (cast `/Game/FBX/Monstre/Volant/ABP_Volant` (`SkeletalMeshComponent.GetAnimInstance` (`self.Mesh`))))
  (set `self.Anim` _asabp_volant)
  (`self.AddToPivotAndCollider` (`self.Sphere_0`)))

(event `self.ReceiveTick`
  (params (DeltaSeconds :type "Float (single-precision)"))
  (`parent.ReceiveTick` DeltaSeconds)
  (if (> (`self.LifePoint`) 0.0)
    (`self.RotateTowardDir`)))

(event `self.CapsuleComponent.OnComponentHit`
  (params (HitComponent :type "PrimitiveComponent Object Reference") (OtherActor :type "Actor Object Reference") (OtherComp :type "PrimitiveComponent Object Reference") (NormalImpulse :type "Vector Structure") (Hit :type "HitResult Structure (by ref)"))
  (if (`|EnumEquality` (`self.State`) "NewEnumerator2")
    (`/Engine/EditorBlueprintResources/StandardMacros.DoOnce` false :!label _label
      (:`Completed`
        (bind _asbp_player (cast `/Game/BluePrint/Entity/BP_Player` OtherActor))
        (`/Game/BluePrint/Entity/BP_Player.LoseLife` _asbp_player true (`SceneComponent.K2_GetComponentLocation` (`self.CapsuleComponent`)) OtherActor)))
    (else
      (goto _label :!via `Reset`))))

(event `self.StartState`
  (switch `/Game/BluePrint/Entity/Enemy/E_EnemyState` (`self.State`)))

(fn `ChangeMatLifeColor`
  (`MaterialInstanceDynamic.SetScalarParameterValue` (`self.MatVolant`) "HeatDissolve" (`KismetMathLibrary.FClamp` (/ (`self.LifePoint`) (`self.MaxLife`)))))

(fn `DamagePlace`
  (params (TouchedPart :type "HitResult Structure") (Damage :type "Float (double-precision)") (Laser :type Boolean))
  (bind _anim (`self.Anim`))
  (`parent.DamagePlace` TouchedPart Damage false)
  (if Laser
    (set `/Game/FBX/Monstre/Volant/ABP_Volant.IsDamageLaser` true _anim)
    (else
      (set `/Game/FBX/Monstre/Volant/ABP_Volant.IsDamageGun` true _anim))))

(fn `Death`
  (`parent.Death`)
  (set `/Game/FBX/Monstre/Volant/ABP_Volant.IsDead` true (`self.Anim`)))

(fn `Death Delay`
  (params (deltaTime :type "Float (double-precision)"))
  (bind _timerdeath (`self.TimerDeath`))
  (if (!= _timerdeath -1.0)
    (bind _returnvalue (`FFMathBlueprintHelper.IncrementFloat` _timerdeath deltaTime))
    (bind _returnvalue_2 (`KismetMathLibrary.Abs` (- (`KismetMathLibrary.FClamp` (/ _returnvalue (`.EnemyDeathSpeed_51_25410B914FA95D940827A6A4B502FA4F` (break `/Game/BluePrint/Data/S_Enemy` (`self.controlVar`))))) 1.0)))
    (`MaterialInstanceDynamic.SetScalarParameterValue` (`self.MatVolant`) "DeathDissolve" _returnvalue_2)
    (`MaterialInstanceDynamic.SetScalarParameterValue` (`self.Mat light`) "DeathDissolve" _returnvalue_2)
    (if (> (`self.TimerDeath`) (`.EnemyDeathSpeed_51_25410B914FA95D940827A6A4B502FA4F` (break `/Game/BluePrint/Data/S_Enemy` (`self.controlVar`))))
      (`self.K2_DestroyActor` self))))

(fn `GetPath`
  (params (ToGO :type "Vector Structure") (ClearPath :type Boolean))
  (returns (Point :type "Vector Structure"))
  (locals (LocalGoTo :type "Vector Structure"))
  (if (not ClearPath)
    (`/Engine/EditorBlueprintResources/StandardMacros.IsValid` (`self.NavMesh`)
      (:`Is Valid`
        (if (not (!= (`KismetArrayLibrary.Array_Length` (`self.NodePath`)) 0))
          (bind _returnvalue (`FFNavMeshEnemy.FindPath` (`self.NavMesh`) (`SceneComponent.K2_GetComponentLocation` (`self.CapsuleComponent`)) ToGO))
          (set `self.NodePath` _returnvalue))
        (set `local.LocalGoTo` (`|GetArrayItem` (`self.NodePath`)))
        (`KismetArrayLibrary.Array_Remove` (`self.NodePath`))
        (return (`local.LocalGoTo`)))
      (:`Is Not Valid`
        (return (69.0 420.0 1312.0))))
    (else
      (`KismetArrayLibrary.Array_Clear` (`self.NodePath`)))))

(fn `RotateTowardDir`
  (if (or (`|EnumEquality` (`self.State`) "NewEnumerator2") (`|EnumEquality` (`self.State`) "NewEnumerator0"))
    (`SceneComponent.K2_SetWorldRotation` (`self.Pivot`) (`KismetMathLibrary.FindLookAtRotation` (`KismetMathLibrary.MakeVector` (.x (`self.prevPos`)) (.y (`self.prevPos`))) (`KismetMathLibrary.MakeVector` (.x (`SceneComponent.K2_GetComponentLocation` (`self.CapsuleComponent`))) (.y (`SceneComponent.K2_GetComponentLocation` (`self.CapsuleComponent`))))) false false)
    (set `self.prevPos` (`SceneComponent.K2_GetComponentLocation` (`self.CapsuleComponent`)))
    (else
      (`SceneComponent.K2_SetWorldRotation` (`self.Pivot`) (`KismetMathLibrary.FindLookAtRotation` (`SceneComponent.K2_GetComponentLocation` (`self.CapsuleComponent`)) (`SceneComponent.K2_GetComponentLocation` (`/Game/BluePrint/Entity/BP_Player.PlayerCol` (`self.Player`)))) false false))))

(fn `StayUp`
  (params (Alpha :type "Float (single-precision)"))
  (bind _capsulecomponent (`self.CapsuleComponent`))
  (bind _returnvalue (`SceneComponent.K2_GetComponentLocation` _capsulecomponent))
  (if (not (`|EnumEquality` (`self.State`) "NewEnumerator2"))
    (`SceneComponent.K2_SetWorldLocation` _capsulecomponent (`KismetMathLibrary.VLerp` _returnvalue (`KismetMathLibrary.MakeVector` (.x _returnvalue) (.y _returnvalue) (+ (.z (`SceneComponent.K2_GetComponentLocation` (`/Game/BluePrint/Entity/BP_Player.PlayerCol` (`self.Player`)))) (`.FlyingHeight_30_FF7BED0946D01A913B070189350F90A5` (break `/Game/BluePrint/Data/S_Enemy` (`self.controlVar`))))) Alpha) false false)))

(fn `UserConstructionScript`
  (`parent.UserConstructionScript`))
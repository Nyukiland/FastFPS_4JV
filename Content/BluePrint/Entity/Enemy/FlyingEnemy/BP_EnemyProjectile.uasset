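; BP_EnemyProjectile is a fireball fired by a flying enemy that costs the player a life on contact.
; SetUp stores the actor to ignore and direction, orients the fireball VFX, and starts a five-second self-destruct.
; Tick sets the sphere's physics velocity along that direction while the ignored actor remains valid.
; Under the same validity check, overlapping any other actor destroys the projectile, calling LoseLife on BP_Player.
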(event `WaitDestroy`
  (`KismetSystemLibrary.Delay` 5.0)
  (`self.K2_DestroyActor`))

(event `self.ReceiveTick`
  (params (DeltaSeconds :type "Float (single-precision)"))
  (`/Engine/EditorBlueprintResources/StandardMacros.IsValid` (`self.actorToIgnore`)
    (:`Is Valid`
      (`PrimitiveComponent.SetPhysicsLinearVelocity` (`self.Sphere`) (* (`self.Dir`) (`self.Speed`)) false "None"))))

(event `self.Sphere.OnComponentBeginOverlap`
  (params (OverlappedComponent :type "PrimitiveComponent Object Reference") (OtherActor :type "Actor Object Reference") (OtherComp :type "PrimitiveComponent Object Reference") (OtherBodyIndex :type Integer) (bFromSweep :type Boolean) (SweepResult :type "HitResult Structure (by ref)"))
  (bind _actortoignore (`self.actorToIgnore`))
  (`/Engine/EditorBlueprintResources/StandardMacros.IsValid` _actortoignore
    (:`Is Valid`
      (if (!= _actortoignore OtherActor)
        (`|ExecutionSequence`
          (:`then_0`
            (bind _asbp_player (cast `/Game/BluePrint/Entity/BP_Player` OtherActor))
            (`/Game/BluePrint/Entity/BP_Player.LoseLife` _asbp_player true))
          (:`then_1`
            (`self.K2_DestroyActor` self)))))))

(fn `SetUp`
  (params (ActorToIgnore :type "Actor Object Reference") (Dir :type "Vector Structure"))
  (bind _returnvalue (`KismetMathLibrary.Normal` Dir))
  (bind _vfx_fireball (`self.VFX_FireBall`))
  (bind _returnvalue_2 (`SceneComponent.K2_GetComponentLocation` _vfx_fireball))
  (set `self.actorToIgnore` ActorToIgnore)
  (set `self.Dir` _returnvalue)
  (`SceneComponent.K2_SetRelativeRotation` _vfx_fireball (`KismetMathLibrary.FindLookAtRotation` _returnvalue_2 (+ _returnvalue_2 _returnvalue)) false false)
  (`self.WaitDestroy`))

(fn `UserConstructionScript`)
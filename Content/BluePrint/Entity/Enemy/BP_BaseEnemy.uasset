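; Base enemy character that registers with the enemy control, loads stats from DT_EnemyDataTable by row name and runs a behavior tree.
; DamagePlace lowers life and returns a value mapped to the hit physical material, while Tick drives a material life lerp.
; Death notifies the control, stops AI, disables collision and destroys the actor on Tick.
; PropelEnemy swaps movement and AI for physics knockback until a downward trace finds ground.
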(event `self.ReceiveBeginPlay`
  (`self.SetUp`)
  (`self.AddToPivotAndCollider` (`self.Mesh`))
  (`KismetArrayLibrary.Array_Add` (`self.ColliderObject`) (`self.CapsuleComponent`)))

(event `self.ReceiveTick`
  (params (DeltaSeconds :type "Float (single-precision)"))
  (`self.ChangeMatLifeColor`)
  (`self.Death Delay` DeltaSeconds)
  (`self.EndPropel`))

(event `StartState`)

(event `TickState`)

(event `Fail`)

(fn `AddToPivotAndCollider`
  (params (Obj :type "PrimitiveComponent Object Reference (by ref)"))
  (`SceneComponent.K2_AttachToComponent` Obj (`self.Pivot`) "None" "KeepRelative" "KeepRelative" "KeepRelative" true)
  (`KismetArrayLibrary.Array_Add` (`self.ColliderObject`) Obj))

(fn `ChangeMatLifeColor`
  (locals (parameter :type Name :default "LerpLife"))
  (for _array_element (`self.MaterialsInstanced`)
    (`MaterialInstanceDynamic.SetScalarParameterValue` _array_element "LerpLife" (`KismetMathLibrary.FClamp` (/ (`self.LifePoint`) (`self.MaxLife`))))))

(fn `DamagePlace`
  (params (TouchedPart :type "HitResult Structure") (Damage :type "Float (double-precision)") (Laser :type Boolean))
  (returns (TouchedBodyPart :type "/Game/BluePrint/Data/E_BodyParts Enum"))
  (bind (_bblockinghit _binitialoverlap _time _distance _location _impactpoint _normal _impactnormal _physmat) (`GameplayStatics.BreakHitResult` TouchedPart))
  (bind _value (`BlueprintMapLibrary.Map_Find` (`self.BodyPartsMap`) _physmat))
  (if (> (`self.LifePoint`) 0.0)
    (`FFMathBlueprintHelper.DecrementFloat` (`self.LifePoint`) Damage)
    (if (<= (`self.LifePoint`) 0)
      (`self.Death`)
      (return _value)
      (else
        (`NiagaraFunctionLibrary.SpawnSystemAtLocation` "/Game/VFX/Ennemi/VFX_EnnemyHurt.VFX_EnnemyHurt" _location (`KismetMathLibrary.FindLookAtRotation` _location _impactnormal))
        (return _value)))))

(fn `Death`
  (bind _returnvalue (`FFEnemyControl.GetEnemyControl` self))
  (`FFEnemyControl.EnemyDied` _returnvalue self)
  (`NiagaraFunctionLibrary.SpawnSystemAtLocation` "/Game/VFX/Ennemi/VFX_EnnemyDeath.VFX_EnnemyDeath" (`SceneComponent.K2_GetComponentLocation` (`self.CapsuleComponent`)))
  (bind _asbp_aicontroller (cast `/Game/BluePrint/Entity/Enemy/BP_AIController` (`AIBlueprintHelperLibrary.GetAIController` self)))
  (bind _braincomponent (`AIController.BrainComponent` _asbp_aicontroller))
  (`/Engine/EditorBlueprintResources/StandardMacros.IsValid` _braincomponent
    (:`Is Valid`
      (`BrainComponent.StopLogic` _braincomponent "Death"))
    (:`Is Not Valid`
      _))
  (`ActorComponent.Deactivate` (`self.CharacterMovement`))
  (`PrimitiveComponent.SetPhysicsLinearVelocity` (`self.CapsuleComponent`) (0.0 0.0 0.0) false "None")
  (set `self.State` "NewEnumerator3")
  (set `self.TimerDeath` 0.0)
  (for _array_element (`self.ColliderObject`)
    (`PrimitiveComponent.SetCollisionEnabled` _array_element "NoCollision")))

(fn `Death Delay`
  (params (deltaTime :type "Float (double-precision)"))
  (if (!= (`self.TimerDeath`) -1.0)
    (`self.K2_DestroyActor` self)))

(fn `EndPropel`
  (bind _returnvalue (`SceneComponent.K2_GetComponentLocation` (`self.CapsuleComponent`)))
  (if (`self.InPropel`)
    (bind _returnvalue_2 (`FFEnemyControl.GetEnemyControl` self))
    (bind _returnvalue_3 (`FFEnemyControl.GetAllEnemies` _returnvalue_2))
    (bind (_outhit _returnvalue_4) (`KismetSystemLibrary.LineTraceSingle` _returnvalue (+ _returnvalue (`KismetMathLibrary.MakeVector` 0.0 0.0 (* (+ (`CapsuleComponent.GetScaledCapsuleHalfHeight` (`self.CapsuleComponent`)) 2.0) -1.0))) "TraceTypeQuery1" false _returnvalue_3))
    (if _returnvalue_4
      (set `self.InPropel` false)
      (`ActorComponent.Activate` (`self.CharacterMovement`) false)
      (`PrimitiveComponent.SetSimulatePhysics` (`self.CapsuleComponent`) false)
      (bind _asbp_aicontroller (cast `/Game/BluePrint/Entity/Enemy/BP_AIController` (`AIBlueprintHelperLibrary.GetAIController` self)))
      (`AIController.RunBehaviorTree` _asbp_aicontroller (`self.BehaviorTree`)))))

(fn `LineTraceMoveForward`
  (params (Dir :type "Vector Structure"))
  (returns (IsHit :type Boolean))
  (locals (tempStored :type "Array of Actor Object Reference") (DistCheck :type "Float (double-precision)" :default 100.0))
  (bind _returnvalue (`SceneComponent.K2_GetComponentLocation` (`self.CapsuleComponent`)))
  (bind _returnvalue_2 (`FFEnemyControl.GetEnemyControl` self))
  (bind _returnvalue_3 (`FFEnemyControl.GetAllEnemies` _returnvalue_2))
  (bind _output_get (set `local.tempStored` _returnvalue_3))
  (`KismetArrayLibrary.Array_Add` _output_get (`self.Player`))
  (bind (_outhit _returnvalue_4) (`KismetSystemLibrary.LineTraceSingle` _returnvalue (+ _returnvalue (* (`KismetMathLibrary.Normal` Dir) (`local.DistCheck`))) "TraceTypeQuery1" false (`local.tempStored`)))
  (return _returnvalue_4))

(fn `PropelEnemy`
  (params (properlPos :type "Vector Structure") (MaxPropelDist :type "Float (double-precision)"))
  (bind _capsulecomponent (`self.CapsuleComponent`))
  (bind _returnvalue (`SceneComponent.K2_GetComponentLocation` (`self.CapsuleComponent`)))
  (bind _asbp_aicontroller (cast `/Game/BluePrint/Entity/Enemy/BP_AIController` (`AIBlueprintHelperLibrary.GetAIController` self)))
  (bind _braincomponent (`AIController.BrainComponent` _asbp_aicontroller))
  (`/Engine/EditorBlueprintResources/StandardMacros.IsValid` _braincomponent
    (:`Is Valid`
      (`BrainComponent.StopLogic` _braincomponent "hold")
      (`ActorComponent.Deactivate` (`self.CharacterMovement`))
      (`PrimitiveComponent.SetSimulatePhysics` _capsulecomponent true)
      (`SceneComponent.K2_AddWorldOffset` _capsulecomponent (0.0 0.0 5.0) false false)
      (`PrimitiveComponent.SetPhysicsLinearVelocity` _capsulecomponent (* (/ (`KismetMathLibrary.Vector_Distance` properlPos _returnvalue) MaxPropelDist) (`.PropelForce_54_7F024D4841D58A60167C6CA7CE54A90F` (break `/Game/BluePrint/Data/S_Enemy` (`self.controlVar`))) (`KismetMathLibrary.Normal` (+ (- _returnvalue properlPos) (0.0 0.0 100.0)))) false "None")
      (set `self.InPropel` true))))

(fn `SetUp`
  (`|ExecutionSequence`
    (:`then_0`
      (bind _asbp_player (cast `/Game/BluePrint/Entity/BP_Player` (`GameplayStatics.GetPlayerPawn` 0)))
      (set `self.Player` _asbp_player)
      (bind _returnvalue (`FFEnemyControl.GetEnemyControl` self))
      (`FFEnemyControl.RegisterEnemySpawned` _returnvalue self)
      (`ActorComponent.Activate` (`self.CharacterMovement`) false))
    (:`then_1`
      (bind _returnvalue_2 (`|GetDataTableRow` "/Game/BluePrint/Data/DT_EnemyDataTable.DT_EnemyDataTable" (`self.EnemyRowName`))
        (:`then`
          (bind _output_get (set `self.controlVar` _returnvalue_2))
          (bind (_enemytype _enemydeathspeed _life _distattack _damage _movementspeed) (break `/Game/BluePrint/Data/S_Enemy` _output_get))
          (bind _output_get_2 (set `self.MaxLife` _life))
          (set `self.LifePoint` _output_get_2)
          (set `CharacterMovementComponent.MaxWalkSpeed` _movementspeed (`self.CharacterMovement`)))))
    (:`then_2`
      (bind _asbp_aicontroller (cast `/Game/BluePrint/Entity/Enemy/BP_AIController` (`AIBlueprintHelperLibrary.GetAIController` self)))
      (`AIController.RunBehaviorTree` _asbp_aicontroller (`self.BehaviorTree`)))))

(fn `UserConstructionScript`)
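; BP_FlyingEnemy is a flying enemy that homes in on the player.
; Each Tick runs the parent tick, calls Move, then rotates the Sphere component to face the player's PlayerCol.
; Move overwrites the Sphere's physics linear velocity with a normalized direction toward a point slightly above PlayerCol, scaled by MovementSpeed.
; It steers in a straight line, with no pathfinding or obstacle avoidance.
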(event `self.ReceiveTick`
  (params (DeltaSeconds :type "Float (single-precision)"))
  (`parent.ReceiveTick` DeltaSeconds)
  (`self.Move`)
  (`SceneComponent.K2_SetWorldRotation` (`self.Sphere`) (`KismetMathLibrary.FindLookAtRotation` (`SceneComponent.K2_GetComponentLocation` (`self.Sphere`)) (`SceneComponent.K2_GetComponentLocation` (`/Game/BluePrint/Entity/BP_Player.PlayerCol` (`self.Player`)))) false false))

(fn `Move`
  (`PrimitiveComponent.SetPhysicsLinearVelocity` (`self.Sphere`) (* (`KismetMathLibrary.Normal` (- (+ (`SceneComponent.K2_GetComponentLocation` (`/Game/BluePrint/Entity/BP_Player.PlayerCol` (`self.Player`))) (0.0 0.0 10.0)) (`SceneComponent.K2_GetComponentLocation` (`self.Sphere`)))) (`self.MovementSpeed`)) false "None"))

(fn `UserConstructionScript`
  (`parent.UserConstructionScript`))
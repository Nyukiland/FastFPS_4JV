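; Enemy projectile actor that damages the player on contact.
; SetUpProjectile stores the damage and a movement vector, and Tick offsets the Sphere component along that vector, scaled by MovementSpeed and delta time, without sweeping.
; On Sphere overlap it calls LoseLife if the other actor is BP_Player, then destroys itself whatever it touched.
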(event `self.ReceiveTick`
  (params (DeltaSeconds :type "Float (single-precision)"))
  (`SceneComponent.K2_AddWorldOffset` (`self.Sphere`) (* (`self.Dir`) (`self.Movement Speed`) DeltaSeconds) false false))

(event `self.Sphere.OnComponentBeginOverlap`
  (params (OverlappedComponent :type "PrimitiveComponent Object Reference") (OtherActor :type "Actor Object Reference") (OtherComp :type "PrimitiveComponent Object Reference") (OtherBodyIndex :type Integer) (bFromSweep :type Boolean) (SweepResult :type "HitResult Structure (by ref)"))
  (`|ExecutionSequence`
    (:`then_0`
      (bind _asbp_player (cast `/Game/BluePrint/Entity/BP_Player` OtherActor))
      (`/Game/BluePrint/Entity/BP_Player.LoseLife` _asbp_player (`self.Damage`)))
    (:`then_1`
      (`self.K2_DestroyActor`))))

(fn `SetUpProjectile`
  (params (PosToGO :type "Vector Structure") (Damage :type "Float (double-precision)"))
  (set `self.Dir` PosToGO)
  (set `self.Damage` Damage))

(fn `UserConstructionScript`)
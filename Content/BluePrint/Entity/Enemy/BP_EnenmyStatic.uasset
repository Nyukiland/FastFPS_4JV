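; Static enemy Blueprint, built from Sphere and Cube components, that prepares its materials at game start.
; After the parent BeginPlay, it creates a dynamic instance of MA_LifeLerp on each component and adds both to the Materials array.
; The material name suggests a life-based visual blend, but nothing in this graph drives it; Tick and overlap events are disabled stubs.
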(event `self.ReceiveBeginPlay`
  (`parent.ReceiveBeginPlay`)
  (bind _returnvalue (`PrimitiveComponent.CreateDynamicMaterialInstance` (`self.Sphere`) 0 "/Game/Materials/MA_LifeLerp.MA_LifeLerp" "None"))
  (`KismetArrayLibrary.Array_Add` (`self.Materials`) _returnvalue)
  (bind _returnvalue_2 (`PrimitiveComponent.CreateDynamicMaterialInstance` (`self.Cube`) 0 "/Game/Materials/MA_LifeLerp.MA_LifeLerp" "None"))
  (`KismetArrayLibrary.Array_Add` (`self.Materials`) _returnvalue_2))

(fn `UserConstructionScript`
  (`parent.UserConstructionScript`))
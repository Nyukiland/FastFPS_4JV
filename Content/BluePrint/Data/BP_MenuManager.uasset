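; Menu manager Blueprint that owns the player's crosshair, main menu, game over and pause widgets and switches between game states.
; InitMenus creates all four widgets hidden in the viewport and hands each a reference to itself and the player.
; StartGame, StopGame and StartPause toggle widget visibility, then set pause, mouse cursor and input mode.
; Restart reloads the current level and resets player life and movement.
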(event `EnterUI`
  (`GameplayStatics.SetGamePaused` true)
  (set `PlayerController.bShowMouseCursor` true (`GameplayStatics.GetPlayerController` 0)))

(event `ExitUI`
  (bind _returnvalue (`GameplayStatics.GetPlayerController` 0))
  (`GameplayStatics.SetGamePaused` false)
  (set `PlayerController.bShowMouseCursor` false _returnvalue)
  (`WidgetBlueprintLibrary.SetInputMode_GameOnly` _returnvalue))

(event `StartGame`
  (params (NewGame :type Boolean))
  (bind _menumanager (`/Game/BluePrint/Entity/BP_Player.MenuManager` (`self.Player`)))
  (`self.ShowCrosshair` _menumanager)
  (`self.HideMenus` _menumanager)
  (`self.HideGameOver` _menumanager)
  (`self.HidePause` _menumanager)
  (`self.ExitUI`)
  (if NewGame
    (`self.Restart`)))

(event `StopGame`
  (bind _menumanager (`/Game/BluePrint/Entity/BP_Player.MenuManager` (`self.Player`)))
  (`self.HideCrosshair` _menumanager)
  (`self.HideMenus` _menumanager)
  (`self.HideGameOver` _menumanager)
  (`self.HidePause` _menumanager)
  (`self.EnterUI`))

(event `StartPause`
  (bind _menumanager (`/Game/BluePrint/Entity/BP_Player.MenuManager` (`self.Player`)))
  (`self.HideCrosshair` _menumanager)
  (`self.HideMenus` _menumanager)
  (`self.HideGameOver` _menumanager)
  (`self.ShowPause` _menumanager)
  (`self.EnterUI`))

(event `Restart`
  (bind _player (`self.Player`))
  (`AkGameplayStatics.StopAll`)
  (bind _returnvalue (`GameplayStatics.GetCurrentLevelName` true))
  (`GameplayStatics.OpenLevel` (`KismetStringLibrary.Conv_StringToName` _returnvalue))
  (set `/Game/BluePrint/Entity/BP_Player.PlayerLife` (`/Game/BluePrint/Entity/BP_Player.PlayerMaxLife` _player) _player)
  (`/Game/BluePrint/Entity/BP_MovementComponenet.DelayBegin` (`/Game/BluePrint/Entity/BP_Player.BP_MovementComponent` (`self.Player`))))

(event `ShowCrosshair`
  (`Widget.SetVisibility` (`self.Crosshair`) "Visible")
  (`WidgetBlueprintLibrary.SetInputMode_GameOnly` (`GameplayStatics.GetPlayerController` 0)))

(event `HideCrosshair`
  (`Widget.SetVisibility` (`self.Crosshair`) "Hidden"))

(event `ShowMenus`
  (`Widget.SetVisibility` (`self.MainMenu`) "Visible")
  (`WidgetBlueprintLibrary.SetInputMode_UIOnlyEx` (`GameplayStatics.GetPlayerController` 0) (`self.MainMenu`)))

(event `HideMenus`
  (`Widget.SetVisibility` (`self.MainMenu`) "Hidden"))

(event `ShowGameOver`
  (`Widget.SetVisibility` (`self.GameOver`) "Visible")
  (`WidgetBlueprintLibrary.SetInputMode_UIOnlyEx` (`GameplayStatics.GetPlayerController` 0) (`self.GameOver`)))

(event `HideGameOver`
  (`Widget.SetVisibility` (`self.GameOver`) "Hidden"))

(event `ShowPause`
  (`Widget.SetVisibility` (`self.Pause`) "Visible")
  (`WidgetBlueprintLibrary.SetInputMode_UIOnlyEx` (`GameplayStatics.GetPlayerController` 0) (`self.Pause`))
  (`/Game/Interface/W_PauseMenu.UpdateGodMod` (`self.Pause`)))

(event `HidePause`
  (`Widget.SetVisibility` (`self.Pause`) "Hidden"))

(fn `InitMenus`
  (params (Player :type "/Game/BluePrint/Entity/BP_Player Object Reference"))
  (bind _output_get (set `self.Player` Player))
  ;[1 1 1] Crosshair
  (bind _returnvalue (`|CreateWidget` "/Game/Interface/W_Crosshair.W_Crosshair_C"))
  (bind _output_get_2 (set `self.Crosshair` _returnvalue))
  (`UserWidget.AddToViewport` _output_get_2 0)
  (set `/Game/Interface/W_Crosshair.MenuManager` self _output_get_2)
  (set `/Game/Interface/W_Crosshair.Player` _output_get _output_get_2)
  (`/Game/Interface/W_Crosshair.InitComboValues` _output_get_2)
  (`Widget.SetVisibility` _output_get_2 "Hidden")
  ;[1 1 1] Main menu
  (bind _returnvalue_2 (`|CreateWidget` "/Game/Interface/W_MainMenu.W_MainMenu_C"))
  (bind _output_get_3 (set `self.MainMenu` _returnvalue_2))
  (`UserWidget.AddToViewport` _output_get_3 0)
  (set `/Game/Interface/W_MainMenu.MenuManager` self _output_get_3)
  (set `/Game/Interface/W_MainMenu.Player` _output_get _output_get_3)
  (`Widget.SetVisibility` _output_get_3 "Hidden")
  ;[1 1 1] GameOver
  (bind _returnvalue_3 (`|CreateWidget` "/Game/Interface/W_GameOver.W_GameOver_C"))
  (bind _output_get_4 (set `self.GameOver` _returnvalue_3))
  (`UserWidget.AddToViewport` _output_get_4 0)
  (set `/Game/Interface/W_GameOver.MenuManager` self _output_get_4)
  (set `/Game/Interface/W_GameOver.Player` _output_get _output_get_4)
  (`Widget.SetVisibility` _output_get_4 "Hidden")
  ;[1 1 1] Pause
  (bind _returnvalue_4 (`|CreateWidget` "/Game/Interface/W_PauseMenu.W_PauseMenu_C"))
  (bind _output_get_5 (set `self.Pause` _returnvalue_4))
  (`UserWidget.AddToViewport` _output_get_5 0)
  (set `/Game/Interface/W_PauseMenu.MenuManager` self _output_get_5)
  (set `/Game/Interface/W_PauseMenu.Player` _output_get _output_get_5)
  (`Widget.SetVisibility` _output_get_5 "Hidden"))

(fn `UserConstructionScript`)
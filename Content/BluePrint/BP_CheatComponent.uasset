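; Cheat and easter egg component that turns held key combinations into debug actions on BP_Player.
; Key events set per-key booleans, which Tick checks while Right Shift is held: kill all enemies, toggle god mode, or reload the level.
; Adding Left Alt instead shows a yogurt widget or spawns a slime, each removed once its combo breaks.
; God mode refills health and ammo every tick; TPPlayer is defined but never called.
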(event `self.ReceiveBeginPlay`
  (bind _returnvalue (`GameplayStatics.GetActorOfClass` "/Game/BluePrint/Entity/BP_Player.BP_Player_C"))
  (set `self.Player` _returnvalue))

(event `self.ReceiveTick`
  (params (DeltaSeconds :type "Float (single-precision)"))
  (bind _player (`self.Player`))
  (bind _currentweapon (`/Game/BluePrint/Entity/BP_WeaponComponent.CurrentWeapon` (`/Game/BluePrint/Entity/BP_Player.BP_WeaponComponent` (`self.Player`))))
  (`|ExecutionSequence`
    (:`then_0`
      ;[1 1 1] Input Management
      (if (`self.Shift`)
        (if (`self.Alt`)
          (`self.EasterEgg`)
          (else
            (`self.Cheat`)))))
    (:`then_1`
      (if (`self.IsGodMod`)
        (set `/Game/BluePrint/Entity/BP_Player.PlayerLife` (`/Game/BluePrint/Entity/BP_Player.PlayerMaxLife` _player) _player)
        (set `/Game/BluePrint/Weapon/BP_WeaponBase.AmunitionsLeft` (`.BulletsQuantity_45_ABF44989497190159D8D86BF3505FBC6` (break `/Game/BluePrint/Data/S_Weapon` (`/Game/BluePrint/Weapon/BP_WeaponBase.WeaponData` _currentweapon))) _currentweapon)))))

(event `Key|A`
  (params (Key :type "Key Structure"))
  (:`Pressed`
    (set `self.A` true))
  (:`Released`
    (set `self.A` false)))

(event `Key|F`
  (params (Key :type "Key Structure"))
  (:`Pressed`
    (set `self.F` true))
  (:`Released`
    (set `self.F` false)))

(event `Key|K`
  (params (Key :type "Key Structure"))
  (:`Pressed`
    (set `self.K` true))
  (:`Released`
    (set `self.K` false)))

(event `Key|P`
  (params (Key :type "Key Structure"))
  (:`Pressed`
    (set `self.P` true))
  (:`Released`
    (set `self.P` false)))

(event `Key|U`
  (params (Key :type "Key Structure"))
  (:`Pressed`
    (set `self.U` true))
  (:`Released`
    (set `self.U` false)))

(event `Key|Z`
  (params (Key :type "Key Structure"))
  (:`Pressed`
    (set `self.Z` true))
  (:`Released`
    (set `self.Z` false)))

(event `Key|B`
  (params (Key :type "Key Structure"))
  (:`Pressed`
    (set `self.B` true))
  (:`Released`
    (set `self.B` false)))

(event `Key|G`
  (params (Key :type "Key Structure"))
  (:`Pressed`
    (set `self.G` true))
  (:`Released`
    (set `self.G` false)))

(event `Key|L`
  (params (Key :type "Key Structure"))
  (:`Pressed`
    (set `self.L` true))
  (:`Released`
    (set `self.L` false)))

(event `Key|Q`
  (params (Key :type "Key Structure"))
  (:`Pressed`
    (set `self.Q` true))
  (:`Released`
    (set `self.Q` false)))

(event `Key|V`
  (params (Key :type "Key Structure"))
  (:`Pressed`
    (set `self.V` true))
  (:`Released`
    (set `self.V` false)))

(event `Key|RightShift`
  (params (Key :type "Key Structure"))
  (:`Pressed`
    (set `self.Shift` true))
  (:`Released`
    (set `self.Shift` false)))

(event `Key|LeftAlt`
  (params (Key :type "Key Structure"))
  (:`Pressed`
    (set `self.Alt` true))
  (:`Released`
    (set `self.Alt` false)))

(event `Key|C`
  (params (Key :type "Key Structure"))
  (:`Pressed`
    (set `self.C` true))
  (:`Released`
    (set `self.C` false)))

(event `Key|H`
  (params (Key :type "Key Structure"))
  (:`Pressed`
    (set `self.H` true))
  (:`Released`
    (set `self.H` false)))

(event `Key|M`
  (params (Key :type "Key Structure"))
  (:`Pressed`
    (set `self.M` true))
  (:`Released`
    (set `self.M` false)))

(event `Key|R`
  (params (Key :type "Key Structure"))
  (:`Pressed`
    (set `self.R` true))
  (:`Released`
    (set `self.R` false)))

(event `Key|W`
  (params (Key :type "Key Structure"))
  (:`Pressed`
    (set `self.W` true))
  (:`Released`
    (set `self.W` false)))

(event `Key|D`
  (params (Key :type "Key Structure"))
  (:`Pressed`
    (set `self.D` true))
  (:`Released`
    (set `self.D` false)))

(event `Key|I`
  (params (Key :type "Key Structure"))
  (:`Pressed`
    (set `self.I` true))
  (:`Released`
    (set `self.I` false)))

(event `Key|N`
  (params (Key :type "Key Structure"))
  (:`Pressed`
    (set `self.N` true))
  (:`Released`
    (set `self.N` false)))

(event `Key|S`
  (params (Key :type "Key Structure"))
  (:`Pressed`
    (set `self.S` true))
  (:`Released`
    (set `self.S` false)))

(event `Key|X`
  (params (Key :type "Key Structure"))
  (:`Pressed`
    (set `self.X` true))
  (:`Released`
    (set `self.X` false)))

(event `Key|E`
  (params (Key :type "Key Structure"))
  (:`Pressed`
    (set `self.E` true))
  (:`Released`
    (set `self.E` false)))

(event `Key|J`
  (params (Key :type "Key Structure"))
  (:`Pressed`
    (set `self.J` true))
  (:`Released`
    (set `self.J` false)))

(event `Key|O`
  (params (Key :type "Key Structure"))
  (:`Pressed`
    (set `self.O` true))
  (:`Released`
    (set `self.O` false)))

(event `Key|T`
  (params (Key :type "Key Structure"))
  (:`Pressed`
    (set `self.T` true))
  (:`Released`
    (set `self.T` false)))

(event `Key|Y`
  (params (Key :type "Key Structure"))
  (:`Pressed`
    (set `self.Y` true))
  (:`Released`
    (set `self.Y` false)))

(fn `Cheat`
  (`self.KillAllEnemies`)
  (`self.GodMod`)
  (`self.QuickReloadScene`))

(fn `EasterEgg`
  (`self.YogurtEasterEgg`)
  (`self.Slime`))

(fn `GodMod`
  (if (`self.G`)
    (if (not (`self.GodDoOnce`))
      (set `self.GodDoOnce` true)
      (set `self.IsGodMod` (not (`self.IsGodMod`))))
    (else
      (set `self.GodDoOnce` false))))

(fn `KillAllEnemies`
  (if (`self.K`)
    (bind _returnvalue (`FFEnemyControl.GetEnemyControl` self))
    (`FFEnemyControl.KillAllEnemies` _returnvalue)))

(fn `QuickReloadScene`
  (if (`self.R`)
    (bind _returnvalue (`GameplayStatics.GetCurrentLevelName` true))
    (`GameplayStatics.OpenLevel` (`KismetStringLibrary.Conv_StringToName` _returnvalue))))

(fn `Slime`
  (bind _slimespawned (`self.SlimeSpawned`))
  (bind _playercol (`/Game/BluePrint/Entity/BP_Player.PlayerCol` (`self.Player`)))
  (if (and (`self.V`) (`self.I`) (`self.K`))
    (`/Engine/EditorBlueprintResources/StandardMacros.IsValid` (`self.SlimeSpawned`)
      (:`Is Not Valid`
        (bind _returnvalue (`|SpawnActorFromClass` "/Game/Import/AllGood/BP_Slime.BP_Slime_C" (`KismetMathLibrary.MakeTransform` (+ (* (`SceneComponent.GetForwardVector` _playercol) (10.0 10.0 10.0)) (`SceneComponent.K2_GetComponentLocation` _playercol))) "Undefined" "MultiplyWithRoot" null null))
        (set `self.SlimeSpawned` _returnvalue)))
    (else
      (`/Engine/EditorBlueprintResources/StandardMacros.IsValid` _slimespawned
        (:`Is Valid`
          (`Actor.K2_DestroyActor` _slimespawned))))))

(fn `TPPlayer`
  (bind _player (`self.Player`))
  (if (`self.P`)
    (`SceneComponent.K2_SetWorldLocation` (`/Game/BluePrint/Entity/BP_Player.PlayerCol` _player) (`/Game/BluePrint/Entity/BP_Player.StartPos` _player) false false)))

(fn `YogurtEasterEgg`
  (bind _yogurtui (`self.YogurtUI`))
  (if (and (`self.Y`) (`self.G`) (`self.T`))
    (`/Engine/EditorBlueprintResources/StandardMacros.IsValid` (`self.YogurtUI`)
      (:`Is Not Valid`
        (bind _returnvalue (`|CreateWidget` "/Game/Interface/AllGood/W_YogurtEasterEgg.W_YogurtEasterEgg_C"))
        (bind _output_get (set `self.YogurtUI` _returnvalue))
        (`UserWidget.AddToViewport` _output_get 0)))
    (else
      (`/Engine/EditorBlueprintResources/StandardMacros.IsValid` _yogurtui
        (:`Is Valid`
          (`Widget.RemoveFromParent` _yogurtui)
          (set `self.YogurtUI` null)
          (`KismetSystemLibrary.CollectGarbage`))))))
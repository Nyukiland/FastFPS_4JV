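; BP_Weapon1 is a weapon Blueprint that takes its stats from a data table and handles reloading.
; On BeginPlay it looks up the row named by its WeaponRow handle and caches it as WeaponData.
; Reload sets IsReloading, refills BullletsLeft from WeaponData.Bullets immediately, then clears the flag after a ReloadDuration delay.
; It contains no firing logic, and its construction script is empty.
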(event `self.ReceiveBeginPlay`
  (bind (_datatable _rowname) (break `DataTableRowHandle` (`self.WeaponRow`)))
  (bind _returnvalue (`|GetDataTableRow` _datatable _rowname)
    (:`then`
      (set `self.WeaponData` _returnvalue))))

(event `Reload`
  (bind (_name _damages _bullets _reloadduration) (break `/Game/BluePrint/Weapon/S_Weapon` (`self.WeaponData`)))
  (set `self.IsReloading` true)
  (set `self.BullletsLeft` _bullets)
  (`KismetSystemLibrary.Delay` _reloadduration)
  (set `self.IsReloading` false))

(fn `UserConstructionScript`)
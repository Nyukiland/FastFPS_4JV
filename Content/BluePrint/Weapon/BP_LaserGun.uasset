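; Laser gun weapon Blueprint that handles the gun's visual feedback: beam, liquid fill, charge and muzzle effects.
; BeginPlay creates dynamic materials for the liquid slot on the skeletal mesh and for the laser beam.
; The player's weapon component supplies combo data that colors the liquid and shifts the beam from green to red as the combo bar fills.
; Exposed functions toggle beam, distortion and arc visibility, set fill level, and restart the particle effects.
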(event `self.ReceiveBeginPlay`
  (bind _returnvalue (`PrimitiveComponent.CreateDynamicMaterialInstance` (`self.SkeletalMesh`) 4 "/Game/Materials/Laser/M_Liquid.M_Liquid" "None"))
  (set `self.FillMat` _returnvalue)
  (bind _returnvalue_2 (`PrimitiveComponent.CreateDynamicMaterialInstance` (`self.TrucPourLeLaser`) 0 "/Game/Materials/Laser/MA_LaserRayon.MA_LaserRayon" "None"))
  (set `self.LaserMat` _returnvalue_2))

(event `UpdateLaserColor`
  (bind _returnvalue (`/Game/BluePrint/Entity/BP_WeaponComponent.Get01ComboBar` (`/Game/BluePrint/Entity/BP_Player.BP_WeaponComponent` (`self.Player`))))
  (`MaterialInstanceDynamic.SetVectorParameterValue` (`self.LaserMat`) "Color" (`KismetMathLibrary.LinearColorLerp` (struct :`G` 1.0 :`B` 0.012555 :`A` 1.0) (struct :`R` 1.0 :`G` 0.033458 :`A` 1.0) _returnvalue)))

(fn `CallLaserCharge`
  (`NiagaraComponent.ResetSystem` (`self.VFX_ChargingLaser`)))

(fn `CallShootEffect`
  (`NiagaraComponent.ResetSystem` (`self.VFX_MuzzleShoot`)))

(fn `Set Fill`
  (params (FillValue :type "Float (double-precision)"))
  (`MaterialInstanceDynamic.SetScalarParameterValue` (`self.FillMat`) "LaserFilling" FillValue)
  (bind _combodata (`/Game/BluePrint/Entity/BP_WeaponComponent.GetComboData` (`/Game/BluePrint/Entity/BP_Player.BP_WeaponComponent` (`self.Player`))))
  (`MaterialInstanceDynamic.SetVectorParameterValue` (`self.FillMat`) "LiquidColor" (`.LevelColor_38_B50572934CDD5F69662B1683BF07C839` (break `/Game/BluePrint/Data/S_Combo` _combodata))))

(fn `Toggle Laser`
  (params (LaserOn :type Boolean))
  (bind _returnvalue (not LaserOn))
  (`SceneComponent.SetHiddenInGame` (`self.TrucPourLeLaser`) _returnvalue true)
  (`SceneComponent.SetHiddenInGame` (`self.VFXLaserDistortion`) _returnvalue true)
  (`SceneComponent.SetHiddenInGame` (`self.ElectricArc`) _returnvalue true))

(fn `UserConstructionScript`
  (`parent.UserConstructionScript`))